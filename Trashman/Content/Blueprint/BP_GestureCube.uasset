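; Magic Leap gesture test actor that spins a cube from hand gestures.
; On BeginPlay it enables player input, configures the static gestures to track and hides the cube.
; Finger gestures set yaw by hand side, while open hand and fist set opposite pitch on either hand, zeroed on release.
; Tick feeds both into RotatingMovement; OK gestures set the cube hidden again, despite being commented as activating it.
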(event EventBeginPlay
  (Input|EnableInput (Game|GetPlayerController 0))
  (Class|MagicLeapHandTrackingFunctionLibrary|SetConfiguration (Variables|Default|GetGestures) "NoFilter" "NoFilter" true)
  (Development|SetHiddeninGame (Variables|Default|GetCube) true false))

(event Collision|EventActorBeginOverlap
  (params (OtherActor :type Actor%20Object%20Reference)))

(event EventTick
  (params (DeltaSeconds :type Float%20%28single-precision%29))
  ;[1 1 1] Update Rotator every tick
  (Variables|/Script/Engine.RotatingMovementComponent|SetRotationRate (Variables|Default|GetRotatingMovement) (Math|Rotator|MakeRotator 0.0 (Variables|Default|GetPitch) (Variables|Default|GetYaw))))

(event Input|KeyboardEvents|MagicLeapLeftOk
  (params (Key :type Key%20Structure))
  ;[1 1 1] Activate static mesh with OK Gesture
  (:Pressed
    (Development|SetHiddeninGame (Variables|Default|GetCube) true false)))

(event Input|KeyboardEvents|MagicLeapRightOk
  (params (Key :type Key%20Structure))
  ;[1 1 1] Activate static mesh with OK Gesture
  (:Pressed
    (Development|SetHiddeninGame (Variables|Default|GetCube) true false)))

(event Input|KeyboardEvents|MagicLeapLeftFinger
  (params (Key :type Key%20Structure))
  ;[1 1 1] Adjust Yaw Rotation with Finger Gesture
  (:Pressed
    (Variables|Default|SetYaw -5e+01))
  (:Released
    (Variables|Default|SetYaw 0.0)))

(event Input|KeyboardEvents|MagicLeapRightFinger
  (params (Key :type Key%20Structure))
  ;[1 1 1] Adjust Yaw Rotation with Finger Gesture
  (:Pressed
    (Variables|Default|SetYaw 5e+01))
  (:Released
    (Variables|Default|SetYaw 0.0)))

(event Input|KeyboardEvents|MagicLeapLeftOpenHand
  (params (Key :type Key%20Structure))
  ;[1 1 1] Open Hand Back
  (:Pressed
    (Variables|Default|SetPitch -5e+01))
  (:Released
    (Variables|Default|SetPitch 0.0)))

(event Input|KeyboardEvents|MagicLeapRightOpenHand
  (params (Key :type Key%20Structure))
  ;[1 1 1] Open Hand Back
  (:Pressed
    (Variables|Default|SetPitch -5e+01))
  (:Released
    (Variables|Default|SetPitch 0.0)))

(event Input|KeyboardEvents|MagicLeapLeftFist
  (params (Key :type Key%20Structure))
  ;[1 1 1] Fist Gestures.
  (:Pressed
    (Variables|Default|SetPitch 5e+01))
  (:Released
    (Variables|Default|SetPitch 0.0)))

(event Input|KeyboardEvents|MagicLeapRightFist
  (params (Key :type Key%20Structure))
  ;[1 1 1] Fist Gestures.
  (:Pressed
    (Variables|Default|SetPitch 5e+01))
  (:Released
    (Variables|Default|SetPitch 0.0)))

(fn ConstructionScript)