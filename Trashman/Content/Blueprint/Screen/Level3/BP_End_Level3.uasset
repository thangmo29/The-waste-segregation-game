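; End-of-level actor for Level 3 that shows the score widgets when the level finishes.
; Every Tick it reads the MyGame game instance; a score of 20 or a timer of -1 stops the level audio, activates its own Audio and shows both widget components, with no once-only guard.
; Any actor overlap clears WidgetVisible1 on the game instance.
; Unconnected leftovers include visibility toggles and a chain destroying food and trash actors.
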(event EventBeginPlay)

(event Collision|EventActorBeginOverlap
  (params (OtherActor :type Actor%20Object%20Reference))
  (bind _asmy_game (Utilities|Casting|CastToMyGame (Game|GetGameInstance)))
  (Variables|/Game/Blueprint/control/Mygame/MyGame.MyGame_C|Setwidget_Visible1 _asmy_game false))

(event EventTick
  (params (DeltaSeconds :type Float%20%28single-precision%29))
  ;[1 1 1] show scorewidget end level after time = 0 and score = 20
  (bind _asmy_game (Utilities|Casting|CastToMyGame (Game|GetGameInstance)))
  (if (== (Variables|/Game/Blueprint/control/Mygame/MyGame.MyGame_C|Getscore_count3 _asmy_game) 20)
    (Audio|Components|Audio|Stop (Variables|/Game/Blueprint/control/Mygame/MyGame.MyGame_C|Getaudio_level3 _asmy_game) :!label _label)
    (Components|Activation|Activate (Variables|Default|GetAudio) false)
    (Rendering|SetVisibility (Variables|Default|GetWidget) true false)
    (elif (== (Variables|/Game/Blueprint/control/Mygame/MyGame.MyGame_C|Gettime_count3 _asmy_game) -1)
      (goto _label))))

(fn ConstructionScript)