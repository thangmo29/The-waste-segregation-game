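; BP_Bin_next is an actor with a HowtoNext component, apparently a "next" object for a how-to screen.
; On BeginPlay it stores its root's world location and caches the first BP_ControlPointer in the level.
; Unreachable logic would play a select sound and open Level1 on a trigger press, and set HowtoNext's mass and gravity.
; Tick is empty, so only that initial caching runs.
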(event EventBeginPlay
  (Variables|Default|SetInitialLocation (Transformation|GetWorldLocation (Variables|Default|GetDefaultSceneRoot)))
  (bind _outactors (Actor|GetAllActorsOfClass "/Game/Blueprint/control/ControllerPointer/Blueprints/BP_ControlPointer.BP_ControlPointer_C"))
  (Variables|Default|SetBPControl%20How (Utilities|Array|Get(acopy) _outactors)))

(event Collision|EventActorBeginOverlap
  (params (OtherActor :type Actor%20Object%20Reference)))

(event EventTick
  (params (DeltaSeconds :type Float%20%28single-precision%29)))

(fn ConstructionScript)