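; BP_Time is a level countdown actor, noted as 90 seconds, that shows the remaining time on its Countdown text.
; A one-second Delay on Tick paces the decrement, and each count is copied to TimeCount1 in the MyGame GameInstance.
; The count is zeroed when time runs out or UpdateItem1 leaves CountAllitem1 at ten or more.
; BeginPlay creates an End_Level1 widget without displaying it here.
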(event EventBeginPlay
  (UserInterface|CreateWidget "/Game/Map/Widget/Level1/End_Level1.End_Level1_C"))

(event Collision|EventActorBeginOverlap
  (params (OtherActor :type Actor%20Object%20Reference)))

(event EventTick
  (params (DeltaSeconds :type Float%20%28single-precision%29))
  ;[1 1 1] Time count 90 sec
  (Utilities|FlowControl|Delay 1.0)
  (Variables|Default|Setcount (- (Variables|Default|Getcount) 1))
  (Rendering|Components|TextRender|SetText (Variables|Default|GetCountdown) (Utilities|Text|ToText(Integer) (Variables|Default|Getcount)))
  (bind _asmy_game (Utilities|Casting|CastToMyGame (Game|GetGameInstance)))
  (Variables|/Game/Blueprint/control/Mygame/MyGame.MyGame_C|Settime_count1 _asmy_game (Variables|Default|Getcount))
  ;[1 1 1] set time = 0 after time count = 0
  (if (<= (Variables|/Game/Blueprint/control/Mygame/MyGame.MyGame_C|Gettime_count1 _asmy_game) 0)
    (bind _output_get (Variables|Default|Setcount 0))
    (Rendering|Components|TextRender|SetText (Variables|Default|GetCountdown) (Utilities|Text|ToText(Integer) _output_get))
    (else
      ;[1 1 1] item = 10 set time = 0
      (Default|UpdateItem1 _asmy_game)
      (if (>= (Variables|/Game/Blueprint/control/Mygame/MyGame.MyGame_C|Getcount_Allitem1 _asmy_game) 10)
        (Variables|Default|Setcount 0)
        (Rendering|Components|TextRender|SetText (Variables|Default|GetCountdown) (Utilities|Text|ToText(Integer) 0))))))

(fn ConstructionScript)