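; Sample player pawn for Magic Leap (Lumin) demo maps, showcasing gaze, hand gestures, controller input and microphone input.
; Flag-gated Tick branches run HMD gaze traces, cache and debug-draw gestures, and sphere-test hand keypoints against InteractionSpheres.
; Tick also broadcasts controller touch axes, while shoulder buttons toggle the main menu and optionally hit-test the world mesh.
; Mic envelope sustained above a threshold fires a one-shot wind event with camera yaw.
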(event Custom|MicInputAudioValue
  (params (EnvelopeValue :type Float%20%28single-precision%29))
  ;[1 0 0 0.5] These are the events used to drive the wind in the Audio and Spatialization map
  (bind _output_get (Variables|MicAndAudio|SetWindEnvelopeValue EnvelopeValue))
  (Math|Float|CompareFloat _output_get (Variables|MicAndAudio|GetWindEnvelopeThreshold)
    (:>
      (Variables|MicandAudio|SetCurrentWindSuccessTime (+ (Variables|MicandAudio|GetCurrentWindSuccessTime) (Utilities|Time|GetWorldDeltaSeconds)) :!label _label)
      (Default|CallWindCheckStarted)
      (Math|Float|CompareFloat (Variables|MicandAudio|GetCurrentWindSuccessTime) (Variables|MicAndAudio|GetWindCheckTimer)
        (:>
          _)
        (:==
          _))
      (Utilities|FlowControl|DoOnce false
        (:Completed
          (Variables|MicandAudio|SetWindEventSuccess true)
          (if (Variables|MicAndAudio|GetWindEventEnabled)
            (Variables|MicandAudio|SetWindEventSuccess true)
            (bind _output_get_2 (Variables|MicAndAudio|SetWorldWindRotation (.yaw (Transformation|GetWorldRotation (Variables|Default|GetCamera)))))
            (Default|CallPlayerWindEvent _output_get_2)))))
    (:==
      (goto _label))
    (:<
      (Variables|MicandAudio|SetCurrentWindSuccessTime 0.0)
      (Default|CallWindCheckFailed))))

(event Custom|StartMicInput
  (bind _audiocapture (Variables|Default|GetAudioCapture))
  ;[1 0 0 0.5] These are the events used to drive the wind in the Audio and Spatialization map
  (CameraShake|Start _audiocapture)
  (Utilities|FlowControl|Delay 1.5)
  (EventDispatchers|BindEventtoOnAudioEnvelopeValue _audiocapture (delegate Custom|MicInputAudioValue))
  (Variables|MicAndAudio|SetWindEventEnabled true)
  (CallFunction|ResetWindTimer)
  (Variables|MicandAudio|SetCurrentWindSuccessTime 0.0))

(event Custom|StopMicInput
  (bind _audiocapture (Variables|Default|GetAudioCapture))
  ;[1 0 0 0.5] These are the events used to drive the wind in the Audio and Spatialization map
  (Audio|Components|Audio|Stop _audiocapture)
  (EventDispatchers|UnbindallEventsfromOnAudioEnvelopeValue _audiocapture)
  (Variables|MicAndAudio|SetWindEventEnabled false))

(event Custom|ResetWindTimer
  ;[1 0 0 0.5] These are the events used to drive the wind in the Audio and Spatialization map
  (Utilities|FlowControl|DoOnce false) ; enters at Reset
)

(event EventBeginPlay
  ;[1 1 1] Gesture Registration. You can change this at runtime
  (Class|MagicLeapHandTrackingFunctionLibrary|SetConfiguration (Utilities|Array|MakeArray "Finger" "Fist" "Pinch" "Thumb" "L" "OpenHandBack" "Ok" "C" "NoHand") "SimpleSmoothing" "MoreRobustnessToFlicker" "SlightRobustnessToFlicker" true))

(event EventTick
  (params (DeltaSeconds :type Float%20%28single-precision%29))
  (Utilities|FlowControl|Sequence
    (:then_0
      ;[1 0.6 0] Implementation Example in PlayerLocationAndGaze.umap
      (if (Variables|PlayerLocationAndGaze|GetUseHMDLookLocation)
        (PlayerLocationAndGaze|CheckHMDLook)))
    (:then_1
      ;[0.2784 1 0] Implementation Example in GesturesAndTotem.umap. See Above for Gesture Registration
      (if (Variables|GesturesAndTotem|GetbCheckForGestures)
        (GesturesAndTotem|UpdateGestures)))
    (:then_2
      ;[0.2784 1 0] Works With GesturesAndTotem.umap. Does Overlap tests for "InteractionSphere" type Actors.
      (if (Variables|GesturesAndTotem|GetbTryTouchOverlap)
        (GesturesandTotem|CheckforGestureInteraction "Left")
        (GesturesandTotem|CheckforGestureInteraction "Right")))
    (:then_3
      ;[0 0.15 1] Event Dispatcher to send data out to our listeners. See MainMenuActor and GesturesandTotem.umap
      (Default|CallPolledTotemTouchAxes (Class|Actor|GetInputAxisKeyValue) (Class|Actor|GetInputAxisKeyValue) (Class|Actor|GetInputAxisKeyValue) (Class|Actor|GetInputAxisKeyValue)))
    (:then_4
      ;[0.4 0 1] This Draws a Transform Widget at the World Origin. Helpful for understanding How your content translates to tracked space
      (if (Variables|Debug|GetbShowWorldOrigin)
        (Rendering|Debug|DrawDebugArrow "0, 0, 0" "5.000000, 0, 0" 1.0 "(R=1.000000,G=0.000000,B=0.000000,A=1.000000)" 0.0 0.5)
        (Rendering|Debug|DrawDebugArrow "0, 0, 0" "0.000000,5.000000, 0" 1.0 "(R=0.000000,G=1.000000,B=0.000000,A=1.000000)" 0.0 0.5)
        (Rendering|Debug|DrawDebugArrow "0, 0, 0" "0.000000, 0,5.000000" 1.0 "(R=0.000000,G=0.000000,B=1.000000,A=1.000000)" 0.0 0.5)))))

(event Input|GamepadEvents|GamepadLeftShoulder
  (params (Key :type Key%20Structure))
  ;[0 0.15 1] Event Dispatcher to send data out to our listeners. See MainMenuActor and GesturesandTotem.umap
  (:Pressed
    (Default|CallShoulderButtonPressed)
    (if (Variables|WorldMeshing|GetbTestWorldHit)
      (WorldMeshing|HitTestWorldMesh))
    (Default|CallToggleMainMenu))
  (:Released
    (Default|CallShoulderButtonReleased)))

(event Input|KeyboardEvents|MotionControllerRightShoulder
  (params (Key :type Key%20Structure))
  ;[0 0.15 1] Event Dispatcher to send data out to our listeners. See MainMenuActor and GesturesandTotem.umap
  (:Pressed
    (Default|CallShoulderButtonPressed)
    (if (Variables|WorldMeshing|GetbTestWorldHit)
      (WorldMeshing|HitTestWorldMesh))
    (Default|CallToggleMainMenu))
  (:Released
    (Default|CallShoulderButtonReleased)))

(fn ConstructionScript)

(fn CheckHMDLook
  (bind _camera (Variables|Default|GetCamera))
  (bind _returnvalue (Transformation|GetWorldLocation _camera))
  ;[1 0.6 0] HMD Look
  (bind _outhit (Collision|LineTraceByChannel _returnvalue (+ _returnvalue (* (Math|Vector|GetForwardVector _camera) 3e+02)) "TraceTypeQuery1" false 0 "None" true "(R=1.000000,G=0.000000,B=0.000000,A=1.000000)" "(R=0.000000,G=1.000000,B=0.000000,A=1.000000)" 0.0))
  ;[1 1 1] PlayerLocationAndGaze.umap
  (bind _aslumin_drone (Utilities|Casting|CastToLumin_Drone (|Hit _outhit)))
  (Variables|/Game/LuminSampleContent/PlayerLocationAndGaze/Blueprints/Lumin_Drone.Lumin_Drone_C|SetbPlayerIsLooking _aslumin_drone true))

(fn UpdateGestures
  (Utilities|FlowControl|Sequence
    (:then_0
      ;[0.2784 1 0] Cache Gestures
      (bind _gesture (Class|MagicLeapHandTrackingFunctionLibrary|GetCurrentGesture "Left"))
      (Variables|GesturesAndTotem|SetCurrentLeftGesture _gesture))
    (:then_1
      (bind _gesture_2 (Class|MagicLeapHandTrackingFunctionLibrary|GetCurrentGesture "Right"))
      (Variables|GesturesAndTotem|SetCurrentRightGesture _gesture_2))
    (:then_2
      (if (and (Utilities|Enum|NotEqual(Enum) (Variables|GesturesAndTotem|GetCurrentLeftGesture) "NoHand") (Variables|Debug|GetbShowGestureDebug))
        (bind _enumvalue (|ForEachEHandTrackingKeypoint)
          (:LoopBody
            (bind (_transform _returnvalue) (Class|MagicLeapHandTrackingFunctionLibrary|GetGestureKeypointTransform "Left" _enumvalue "World"))
            (if _returnvalue
              (Rendering|Debug|DrawDebugSphere (.Location (Math|Transform|BreakTransform _transform)) 1.0 12 (|GestureColorLookUp (Variables|GesturesAndTotem|GetCurrentLeftGesture)) 0.0)))
          (:then
            (bind _handcenter (Class|MagicLeapHandTrackingFunctionLibrary|GetHandCenter "Left"))
            (if true
              (Rendering|Debug|DrawDebugSphere (.Location (Math|Transform|BreakTransform _handcenter)) 1.0 12 "(R=0.000000,G=1.000000,B=0.384554,A=1.000000)" 0.0))))))
    (:then_3
      (if (and (Utilities|Enum|NotEqual(Enum) (Variables|GesturesAndTotem|GetCurrentRightGesture) "NoHand") (Variables|Debug|GetbShowGestureDebug))
        (bind _enumvalue_2 (|ForEachEHandTrackingKeypoint)
          (:LoopBody
            (bind (_transform_2 _returnvalue_2) (Class|MagicLeapHandTrackingFunctionLibrary|GetGestureKeypointTransform "Right" _enumvalue_2 "World"))
            (if _returnvalue_2
              (Rendering|Debug|DrawDebugSphere (.Location (Math|Transform|BreakTransform _transform_2)) 1.0 12 (|GestureColorLookUp_2 (Variables|GesturesAndTotem|GetCurrentLeftGesture)) 0.0)))
          (:then
            (bind (_handcenter_2 _returnvalue_3) (Class|MagicLeapHandTrackingFunctionLibrary|GetHandCenter "Right"))
            (if _returnvalue_3
              (Rendering|Debug|DrawDebugSphere (.Location (Math|Transform|BreakTransform _handcenter_2)) 1.0 12 "(R=0.000000,G=1.000000,B=0.384554,A=1.000000)" 0.0))))))))

(fn CheckforGestureInteraction
  (params (Hand :type EControllerHand%20Enum :default "Left"))
  ;[1 1 1] Doing a quick SphereOverlap test on Gesture Poins. This Actor is in GesturesAndTotem,umap
  (bind _enumvalue (|ForEachEHandTrackingKeypoint)
    (:LoopBody
      (bind (_transform _returnvalue) (Class|MagicLeapHandTrackingFunctionLibrary|GetGestureKeypointTransform Hand _enumvalue "World"))
      (if _returnvalue
        (bind _outactors (Collision|SphereOverlapActors (.Location (Math|Transform|BreakTransform _transform)) 1.0 (Utilities|Array|MakeArray "ObjectTypeQuery1" "ObjectTypeQuery2") "/Game/LuminSampleContent/GesturesAndTotem/Blueprints/InteractionSphere.InteractionSphere_C"))
        (for _array_element _outactors
          (bind _asinteraction_sphere (Utilities|Casting|CastToInteractionSphere _array_element))
          (Variables|/Game/LuminSampleContent/GesturesAndTotem/Blueprints/InteractionSphere.InteractionSphere_C|SetbIsTouched _asinteraction_sphere true))))))

(fn HitTestWorldMesh
  (bind _returnvalue (Math|Random|RandomUnitVector))
  (bind _camera (Variables|Default|GetCamera))
  (bind _returnvalue_2 (Math|Conversions|ToLinearColor(Vector) _returnvalue))
  (bind _returnvalue_3 (Transformation|GetWorldLocation _camera))
  (bind _outhit (Collision|LineTraceByChannel _returnvalue_3 (+ _returnvalue_3 (* (Math|Vector|GetForwardVector _camera) 3e+02)) "TraceTypeQuery1" false 0 "None" true "(R=1.000000,G=0.000000,B=0.000000,A=1.000000)" "(R=0.000000,G=1.000000,B=0.000000,A=1.000000)" 0.0))
  (Utilities|Casting|CastToLuminMeshActor (.HitActor (Collision|BreakHitResult _outhit)))
  (Rendering|Debug|DrawDebugSphere (.ImpactPoint (Collision|BreakHitResult _outhit)) 1.0 12 _returnvalue_2 1e+01)
  (Rendering|Debug|DrawDebugArrow (.ImpactPoint (Collision|BreakHitResult _outhit)) (+ (.ImpactPoint (Collision|BreakHitResult _outhit)) (* (.ImpactNormal (Collision|BreakHitResult _outhit)) 5.0)) 2.0 _returnvalue_2 1e+01 0.0))