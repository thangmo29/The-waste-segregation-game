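; BP_HandTracking is an actor that visualizes left-hand gesture tracking with a small sphere.
; BeginPlay enables player input and configures the static gestures to detect with simple keypoint smoothing.
; Each Tick reads the world-space thumb tip, index tip and hand center in sequence, but all three move the same SphereThumb component, so it ends each frame at the hand center.
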(event EventBeginPlay
  (Input|EnableInput (Game|GetPlayerController 0))
  (Class|MagicLeapHandTrackingFunctionLibrary|SetConfiguration (Variables|Default|GetGestures) "SimpleSmoothing" "NoFilter" true))

(event Collision|EventActorBeginOverlap
  (params (OtherActor :type Actor%20Object%20Reference)))

(event EventTick
  (params (DeltaSeconds :type Float%20%28single-precision%29))
  (Utilities|FlowControl|Sequence
    (:then_0
      (bind _transform (Class|MagicLeapHandTrackingFunctionLibrary|GetGestureKeypointTransform "Left" "Thumb_Tip" "World"))
      (Transformation|SetWorldTransform (Variables|Default|GetSphereThumb) (Math|Transform|MakeTransform (.location _transform) "0, 0, 0" "0.020000,0.020000,0.020000") false false))
    (:then_1
      (bind _transform_2 (Class|MagicLeapHandTrackingFunctionLibrary|GetGestureKeypointTransform "Left" "Index_Tip" "World"))
      (Transformation|SetWorldTransform (Variables|Default|GetSphereThumb) (Math|Transform|MakeTransform (.location _transform_2) "0, 0, 0" "0.020000,0.020000,0.020000") false false))
    (:then_2
      (bind _transform_3 (Class|MagicLeapHandTrackingFunctionLibrary|GetGestureKeypointTransform "Left" "Hand_Center" "World"))
      (Transformation|SetWorldTransform (Variables|Default|GetSphereThumb) (Math|Transform|MakeTransform (.location _transform_3) "0, 0, 0" "0.020000,0.020000,0.020000") false false))))

(fn ConstructionScript)