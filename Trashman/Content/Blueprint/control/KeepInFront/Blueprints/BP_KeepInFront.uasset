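; KeepInFront actor that follows the player's view, staying in front of the camera and settling onto surfaces it looks at.
; Each tick, a camera line trace places it on hits within MaxDistance, shrinking with proximity, otherwise at MaxDistance facing the camera.
; Surface rotation uses the grid-snapped impact normal, or turns toward the camera on horizontal surfaces when MatchGravity is set.
; Transform interpolation adds lag, with positional offsets applied.
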(event EventTick
  (params (DeltaSeconds :type Float%20%28single-precision%29))
  (bind _returnvalue (Game|GetPlayerCameraManager 0))
  (bind _returnvalue_2 (Game|GetPlayerCameraManager 0))
  (bind _anchor (Variables|Default|GetAnchor))
  (bind _returnvalue_3 (Transformation|GetWorldLocation _anchor))
  (bind _transformcomponent (Variables|/Script/Engine.PlayerCameraManager|GetTransformComponent _returnvalue_2))
  (bind _transformcomponent_2 (Variables|/Script/Engine.PlayerCameraManager|GetTransformComponent _returnvalue))
  (bind _returnvalue_4 (Transformation|GetWorldLocation _transformcomponent))
  (bind _returnvalue_5 (Transformation|GetWorldLocation _transformcomponent_2))
  (bind _returnvalue_6 (Math|Rotator|FindLookatRotation _returnvalue_5 _returnvalue_3))
  (bind (_roll _pitch _yaw) (Math|Rotator|BreakRotator _returnvalue_6))
  (bind _returnvalue_7 (+ _yaw 1.8e+02))
  (bind _returnvalue_8 (* _pitch -1.0))
  ;[1 1 1] Raycast Request and breakdown
  (bind (_outhit _returnvalue_9) (Collision|LineTraceByChannel _returnvalue_4 (+ _returnvalue_4 (* (Math|Vector|Normalize (Math|Vector|GetForwardVector _transformcomponent)) 5e+02)) "TraceTypeQuery1" false 0 "None"))
  (if _returnvalue_9 ; Did you hit something?
    (if (<= (.Distance (Collision|BreakHitResult _outhit)) (Variables|Default|GetMaxDistance)) ; Was the object hit less than our max distance
      (if (and (Variables|Default|GetMatchGravity) (!= (Math|Float|SnapToGrid(Float) (.pitch (Math|Conversions|RotationFromXVector (.ImpactNormal (Collision|BreakHitResult _outhit)))) 9e+01) 0.0)) ; Is the object we hit a horizontal surface
        ;[1 1 1] Lerp Transforms in order to create Lag
        (bind _output_get (Variables|Default|SetCurrent%20Transform (Math|Transform|MakeTransform (.Location (Collision|BreakHitResult _outhit)) (Math|Rotator|MakeRotator (.roll (Math|Conversions|RotationFromXVector (.ImpactNormal (Collision|BreakHitResult _outhit)))) _returnvalue_8 _returnvalue_7) (Math|Conversions|ToVector(Float) (Math|Float|Clamp(Float) (* (.Distance (Collision|BreakHitResult _outhit)) (Variables|Default|GetminimumScale)) 0.0 0.9)))))
        (Transformation|SetActorRelativeTransform (Math|Transform|MakeTransform (+ (.Location (Math|Transform|BreakTransform (Class|KismetMathLibrary|TInterpto (Transformation|GetActorTransform) _output_get (Utilities|Time|GetWorldDeltaSeconds) (Variables|Default|GetarrivalSpeed)))) (+ (Variables|Default|GetOffset) (Math|Vector|MakeVector (Variables|Default|GetSurface%20Offset) 0.0 0.0))) (.Rotation (Math|Transform|BreakTransform (Class|KismetMathLibrary|TInterpto (Transformation|GetActorTransform) _output_get (Utilities|Time|GetWorldDeltaSeconds) (Variables|Default|GetarrivalSpeed)))) (.Scale (Math|Transform|BreakTransform (Class|KismetMathLibrary|TInterpto (Transformation|GetActorTransform) _output_get (Utilities|Time|GetWorldDeltaSeconds) (Variables|Default|GetarrivalSpeed))))) true false)
        (else
          ;[1 1 1] Lerp Transforms in order to create Lag
          (bind _output_get_2 (Variables|Default|SetCurrent%20Transform (Math|Transform|MakeTransform (.Location (Collision|BreakHitResult _outhit)) (Math|Rotator|MakeRotator (.roll (Math|Conversions|RotationFromXVector (.ImpactNormal (Collision|BreakHitResult _outhit)))) (Math|Float|SnapToGrid(Float) (.pitch (Math|Conversions|RotationFromXVector (.ImpactNormal (Collision|BreakHitResult _outhit)))) 9e+01) (Math|Float|SnapToGrid(Float) (.yaw (Math|Conversions|RotationFromXVector (.ImpactNormal (Collision|BreakHitResult _outhit)))) 15.0)) (Math|Conversions|ToVector(Float) (Math|Float|Clamp(Float) (* (.Distance (Collision|BreakHitResult _outhit)) (Variables|Default|GetminimumScale)) 0.0 0.9)))))
          (Transformation|SetActorRelativeTransform (Math|Transform|MakeTransform (+ (.Location (Math|Transform|BreakTransform (Class|KismetMathLibrary|TInterpto (Transformation|GetActorTransform) _output_get_2 (Utilities|Time|GetWorldDeltaSeconds) (Variables|Default|GetarrivalSpeed)))) (+ (Variables|Default|GetOffset) (Math|Vector|MakeVector (Variables|Default|GetSurface%20Offset) 0.0 0.0))) (.Rotation (Math|Transform|BreakTransform (Class|KismetMathLibrary|TInterpto (Transformation|GetActorTransform) _output_get_2 (Utilities|Time|GetWorldDeltaSeconds) (Variables|Default|GetarrivalSpeed)))) (.Scale (Math|Transform|BreakTransform (Class|KismetMathLibrary|TInterpto (Transformation|GetActorTransform) _output_get_2 (Utilities|Time|GetWorldDeltaSeconds) (Variables|Default|GetarrivalSpeed))))) true false)))
      (else
        ;[1 1 1] Lerp Transforms in order to create Lag
        (bind _output_get_3 (Variables|Default|SetCurrent%20Transform (Math|Transform|MakeTransform (+ _returnvalue_5 (* (Math|Vector|Normalize (Math|Vector|GetForwardVector _transformcomponent_2)) (Variables|Default|GetMaxDistance))) (Math|Rotator|MakeRotator _roll _returnvalue_8 _returnvalue_7)) :!label _label))
        (Transformation|SetActorRelativeTransform (Math|Transform|MakeTransform (+ (.Location (Math|Transform|BreakTransform (Class|KismetMathLibrary|TInterpto (Transformation|GetActorTransform) _output_get_3 (Utilities|Time|GetWorldDeltaSeconds) (Variables|Default|GetarrivalSpeed)))) (+ (Variables|Default|GetOffset) (Math|Vector|MakeVector (Variables|Default|GetSurface%20Offset) 0.0 0.0))) (.Rotation (Math|Transform|BreakTransform (Class|KismetMathLibrary|TInterpto (Transformation|GetActorTransform) _output_get_3 (Utilities|Time|GetWorldDeltaSeconds) (Variables|Default|GetarrivalSpeed)))) (.Scale (Math|Transform|BreakTransform (Class|KismetMathLibrary|TInterpto (Transformation|GetActorTransform) _output_get_3 (Utilities|Time|GetWorldDeltaSeconds) (Variables|Default|GetarrivalSpeed))))) true false)))
    (else
      (goto _label))))

(fn ConstructionScript)

(fn GetPawnVariables
  (bind _outactors (Actor|GetAllActorsOfClass 0))
  (Variables|Default|SetXRPawn 0))