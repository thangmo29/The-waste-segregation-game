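; BP_Yogurt-Bottlee is a labeled, physics-configured yogurt bottle prop that plays audio feedback for pointer-controller interaction in Level1.
; BeginPlay caches the BP_ControlPointer and start position and sets mass, gravity and title; construction creates the dynamic material.
; Tick compares position and trigger state to flag dragging and drive DoOnce-gated drag sounds.
; Overlap events play target sounds, and hits against non-controller actors play a DoOnce-gated collision sound.
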(event OnComponentBeginOverlap(Cube)
  (params (OverlappedComponent :type Primitive%20Component%20Object%20Reference) (OtherActor :type Actor%20Object%20Reference) (OtherComp :type Primitive%20Component%20Object%20Reference) (OtherBodyIndex :type Integer) (bFromSweep :type Boolean) (SweepResult :type Hit%20Result%20Structure%20%28by%20ref%29))
  (Audio|PlaySoundatLocation (Variables|Default|GetTarget%20Begin%20Sound) (Transformation|GetWorldLocation (Variables|Default|GetCube)) "0, 0, 0" 1.0 1.0 0.0 0 0 0))

(event OnComponentEndOverlap(Cube)
  (params (OverlappedComponent :type Primitive%20Component%20Object%20Reference) (OtherActor :type Actor%20Object%20Reference) (OtherComp :type Primitive%20Component%20Object%20Reference) (OtherBodyIndex :type Integer))
  (Audio|PlaySoundatLocation (Variables|Default|GetTarget%20End%20Sound) (Transformation|GetWorldLocation (Variables|Default|GetCube)) "0, 0, 0" 1.0 1.0 0.0 0 0 0))

(event OnComponentHit(Cube)
  (params (HitComponent :type Primitive%20Component%20Object%20Reference) (OtherActor :type Actor%20Object%20Reference) (OtherComp :type Primitive%20Component%20Object%20Reference) (NormalImpulse :type Vector :default "0, 0, 0") (Hit :type Hit%20Result%20Structure%20%28by%20ref%29))
  (if (!= OtherActor (Variables|Default|GetBPController))
    (Utilities|FlowControl|DoOnce false :!label _label
      (:Completed
        (Audio|PlaySoundatLocation (Variables|Default|GetCollisionSound) (Transformation|GetWorldLocation (Variables|Default|GetCube)) "0, 0, 0" 1.0 1.0 0.0 0 0 0)))
    (else
      (goto _label Reset))))

(event EventBeginPlay
  (bind _cube (Variables|Default|GetCube))
  (Variables|Default|SetInitialLocation (Transformation|GetWorldLocation (Variables|Default|GetCube)))
  (bind _outactors (Actor|GetAllActorsOfClass "/Game/Blueprint/control/ControllerPointer/Blueprints/BP_ControlPointer.BP_ControlPointer_C"))
  (Variables|Default|SetBPController (Utilities|Array|Get(acopy) _outactors))
  (Class|PrimitiveComponent|SetMassOverrideinKg _cube "None" (Variables|Default|GetMass) true)
  (Physics|SetEnableGravity _cube (Variables|Default|GetGravity))
  (Rendering|Components|TextRender|SetText (Variables|Default|GetTextRender) (Variables|Default|GetTitle)))

(event EventTick
  (params (DeltaSeconds :type Float%20%28single-precision%29))
  (if (Math|Vector|Equal(Vector) (Variables|Default|GetInitialLocation) (Transformation|GetWorldLocation (Variables|Default|GetCube)) 1.0)
    (if (not (Variables|/Game/Blueprint/control/ControllerPointer/Blueprints/BP_ControlPointer.BP_ControlPointer_C|GetTriggerPressed (Variables|Default|GetBPController)))
      (Utilities|FlowControl|Sequence
        (:then_0
          (Utilities|FlowControl|DoOnce false :!label _label
            (:Completed
              (Audio|PlaySoundatLocation (Variables|Default|GetDrag%20End%20Sound) (Transformation|GetWorldLocation (Variables|Default|GetCube)) "0, 0, 0" 1.0 1.0 0.0 0 0 0))))
        (:then_1
          (goto _label_2 Reset))))
    (else
      (Variables|Default|SetDragging true)
      (Utilities|FlowControl|Sequence
        (:then_0
          (Utilities|FlowControl|DoOnce false :!label _label_2
            (:Completed
              (Audio|PlaySoundatLocation (Variables|Default|GetDrag%20Begin%20Sound) (Variables|Default|GetInitialLocation) "0, 0, 0" 1.0 1.0 0.0 0 0 0))))
        (:then_1
          (goto _label Reset))))))

(fn ConstructionScript
  (bind _returnvalue (Rendering|Material|CreateDynamicMaterialInstance (Variables|Default|GetCube) 0 "/Game/Model/item/Level1/YELLOW/yogurt-bottle/source/M_yougurt.M_yougurt" "None" :!class /Script/Engine.PrimitiveComponent))
  (Variables|Default|SetTarget%20Material _returnvalue)
  (Rendering|Components|TextRender|SetText (Variables|Default|GetTextRender) (Variables|Default|GetTitle)))