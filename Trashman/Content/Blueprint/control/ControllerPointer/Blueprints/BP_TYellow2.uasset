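; Yellow sorting bin for level 2 of a waste-sorting game, destroying recognized items that overlap its Sphere.
; A cast chain identifies each item: yellow recyclables score +1 with a correct sound, green and blue items -1 with a wrong sound.
; Each hit also increments the item count and that item's tally in MyGame.
; Tick casts the GameInstance to MyGame, which overlap reuses, and copies score and item count into it every frame.
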(event OnComponentBeginOverlap(Sphere)
  (params (OverlappedComponent :type Primitive%20Component%20Object%20Reference) (OtherActor :type Actor%20Object%20Reference) (OtherComp :type Primitive%20Component%20Object%20Reference) (OtherBodyIndex :type Integer) (bFromSweep :type Boolean) (SweepResult :type Hit%20Result%20Structure%20%28by%20ref%29))
  ;[1 1 1] set hidden item and -score in count_score (TGreen) and count item
  (bind _asbp_banana (Utilities|Casting|CastToBP_Banana OtherActor)
    (:then
      (Actor|DestroyActor _asbp_banana)
      (Variables|Default|Setcount_score2 (- (Variables|Default|Getcount_score2) 1))
      (Variables|Default|Setcount_item2 (+ (Variables|Default|Getcount_item2) 1))
      ;;[1 1 1] check wrong item
      (Variables|/Game/Blueprint/control/Mygame/MyGame.MyGame_C|Setlevel2_Green_Banana_check (stale EventTick _asmy_game) (+ (Variables|/Game/Blueprint/control/Mygame/MyGame.MyGame_C|Getlevel2_Green_Banana_check (stale EventTick _asmy_game)) 2))
      (Audio|PlaySound2D "/Game/Map/sound/Wiget/wrong2.wrong2" 6.0 1.0 0.0 0 0))
    (:CastFailed
      (bind _asbp_hotdog (Utilities|Casting|CastToBP_Hotdog OtherActor)
        (:then
          (Actor|DestroyActor _asbp_hotdog)
          (Variables|Default|Setcount_score2 (- (Variables|Default|Getcount_score2) 1))
          (Variables|Default|Setcount_item2 (+ (Variables|Default|Getcount_item2) 1))
          (Variables|/Game/Blueprint/control/Mygame/MyGame.MyGame_C|Setlevel2_Green_Hotdog_check (stale EventTick _asmy_game) (+ (Variables|/Game/Blueprint/control/Mygame/MyGame.MyGame_C|Getlevel2_Green_Hotdog_check (stale EventTick _asmy_game)) 2))
          (Audio|PlaySound2D "/Game/Map/sound/Wiget/wrong2.wrong2" 6.0 1.0 0.0 0 0))
        (:CastFailed
          (bind _asbp_orange (Utilities|Casting|CastToBP_Orange OtherActor)
            (:then
              (Actor|DestroyActor _asbp_orange)
              (Variables|Default|Setcount_score2 (- (Variables|Default|Getcount_score2) 1))
              (Variables|Default|Setcount_item2 (+ (Variables|Default|Getcount_item2) 1))
              (Variables|/Game/Blueprint/control/Mygame/MyGame.MyGame_C|Setlevel2_Green_Orange_check (stale EventTick _asmy_game) (+ (Variables|/Game/Blueprint/control/Mygame/MyGame.MyGame_C|Getlevel2_Green_Orange_check (stale EventTick _asmy_game)) 2))
              (Audio|PlaySound2D "/Game/Map/sound/Wiget/wrong2.wrong2" 6.0 1.0 0.0 0 0))
            (:CastFailed
              (bind _asbp_pig__bone (Utilities|Casting|CastToBP_Pig-Bone OtherActor)
                (:then
                  (Actor|DestroyActor _asbp_pig__bone)
                  (Variables|Default|Setcount_score2 (- (Variables|Default|Getcount_score2) 1))
                  (Variables|Default|Setcount_item2 (+ (Variables|Default|Getcount_item2) 1))
                  (Variables|/Game/Blueprint/control/Mygame/MyGame.MyGame_C|Setlevel2_Green_Pig-bone_check (stale EventTick _asmy_game) (+ (Variables|/Game/Blueprint/control/Mygame/MyGame.MyGame_C|Getlevel2_Green_Pig-bone_check (stale EventTick _asmy_game)) 2))
                  (Audio|PlaySound2D "/Game/Map/sound/Wiget/wrong2.wrong2" 6.0 1.0 0.0 0 0))
                (:CastFailed
                  (bind _asbp_strawberry (Utilities|Casting|CastToBP_Strawberry OtherActor)
                    (:then
                      (Actor|DestroyActor _asbp_strawberry)
                      (Variables|Default|Setcount_score2 (- (Variables|Default|Getcount_score2) 1))
                      (Variables|Default|Setcount_item2 (+ (Variables|Default|Getcount_item2) 1))
                      (Variables|/Game/Blueprint/control/Mygame/MyGame.MyGame_C|Setlevel2_Green_Strawberry_check (stale EventTick _asmy_game) (+ (Variables|/Game/Blueprint/control/Mygame/MyGame.MyGame_C|Getlevel2_Green_Strawberry_check (stale EventTick _asmy_game)) 2))
                      (Audio|PlaySound2D "/Game/Map/sound/Wiget/wrong2.wrong2" 6.0 1.0 0.0 0 0))
                    (:CastFailed
                      ;[1 1 1] set hidden item and +score in count_score (TYellow) and count item
                      (bind _asbp_can (Utilities|Casting|CastToBP_Can OtherActor)
                        (:then
                          (Actor|DestroyActor _asbp_can)
                          (Variables|Default|Setcount_score2 (+ (Variables|Default|Getcount_score2) 1))
                          (Variables|Default|Setcount_item2 (+ (Variables|Default|Getcount_item2) 1))
                          (Variables|/Game/Blueprint/control/Mygame/MyGame.MyGame_C|Setlevel2_Yellow_can (stale EventTick _asmy_game) (+ (Variables|/Game/Blueprint/control/Mygame/MyGame.MyGame_C|Getlevel2_Yellow_can (stale EventTick _asmy_game)) 1))
                          (Variables|/Game/Blueprint/control/Mygame/MyGame.MyGame_C|SetCheck_amount_item_Yellow2 (stale EventTick _asmy_game) (+ (Variables|/Game/Blueprint/control/Mygame/MyGame.MyGame_C|GetCheck_amount_item_Yellow2 (stale EventTick _asmy_game)) 1))
                          (Audio|PlaySound2D "/Game/Map/sound/Wiget/correct.correct" 1.0 1.0 0.0 0 0))
                        (:CastFailed
                          (bind _asbp_cardboard_box_2 (Utilities|Casting|CastToBP_Cardboard-box2 OtherActor)
                            (:then
                              (Actor|DestroyActor _asbp_cardboard_box_2)
                              (Variables|Default|Setcount_score2 (+ (Variables|Default|Getcount_score2) 1))
                              (Variables|Default|Setcount_item2 (+ (Variables|Default|Getcount_item2) 1))
                              (Variables|/Game/Blueprint/control/Mygame/MyGame.MyGame_C|Setlevel2_Yellow_Cardboard-box2 (stale EventTick _asmy_game) (+ (Variables|/Game/Blueprint/control/Mygame/MyGame.MyGame_C|Getlevel2_Yellow_Cardboard-box2 (stale EventTick _asmy_game)) 1))
                              (Variables|/Game/Blueprint/control/Mygame/MyGame.MyGame_C|SetCheck_amount_item_Yellow2 (stale EventTick _asmy_game) (+ (Variables|/Game/Blueprint/control/Mygame/MyGame.MyGame_C|GetCheck_amount_item_Yellow2 (stale EventTick _asmy_game)) 1))
                              (Audio|PlaySound2D "/Game/Map/sound/Wiget/correct.correct" 1.0 1.0 0.0 0 0))
                            (:CastFailed
                              (bind _asbp_milk__box (Utilities|Casting|CastToBP_Milk-Box OtherActor)
                                (:then
                                  (Actor|DestroyActor _asbp_milk__box)
                                  (Variables|Default|Setcount_score2 (+ (Variables|Default|Getcount_score2) 1))
                                  (Variables|Default|Setcount_item2 (+ (Variables|Default|Getcount_item2) 1))
                                  (Variables|/Game/Blueprint/control/Mygame/MyGame.MyGame_C|Setlevel2_Yellow_Milk-Box (stale EventTick _asmy_game) (+ (Variables|/Game/Blueprint/control/Mygame/MyGame.MyGame_C|Getlevel2_Yellow_Milk-Box (stale EventTick _asmy_game)) 1))
                                  (Variables|/Game/Blueprint/control/Mygame/MyGame.MyGame_C|SetCheck_amount_item_Yellow2 (stale EventTick _asmy_game) (+ (Variables|/Game/Blueprint/control/Mygame/MyGame.MyGame_C|GetCheck_amount_item_Yellow2 (stale EventTick _asmy_game)) 1))
                                  (Audio|PlaySound2D "/Game/Map/sound/Wiget/correct.correct" 1.0 1.0 0.0 0 0))
                                (:CastFailed
                                  (bind _asbp_soup_can (Utilities|Casting|CastToBP_Soup-can OtherActor)
                                    (:then
                                      (Actor|DestroyActor _asbp_soup_can)
                                      (Variables|Default|Setcount_score2 (+ (Variables|Default|Getcount_score2) 1))
                                      (Variables|Default|Setcount_item2 (+ (Variables|Default|Getcount_item2) 1))
                                      (Variables|/Game/Blueprint/control/Mygame/MyGame.MyGame_C|Setlevel2_Yellow_soup-can (stale EventTick _asmy_game) (+ (Variables|/Game/Blueprint/control/Mygame/MyGame.MyGame_C|Getlevel2_Yellow_soup-can (stale EventTick _asmy_game)) 1))
                                      (Variables|/Game/Blueprint/control/Mygame/MyGame.MyGame_C|SetCheck_amount_item_Yellow2 (stale EventTick _asmy_game) (+ (Variables|/Game/Blueprint/control/Mygame/MyGame.MyGame_C|GetCheck_amount_item_Yellow2 (stale EventTick _asmy_game)) 1))
                                      (Audio|PlaySound2D "/Game/Map/sound/Wiget/correct.correct" 1.0 1.0 0.0 0 0))
                                    (:CastFailed
                                      (bind _asbp_water_bottle_2 (Utilities|Casting|CastToBP_Water-bottle2 OtherActor)
                                        (:then
                                          (Actor|DestroyActor _asbp_water_bottle_2)
                                          (Variables|Default|Setcount_score2 (+ (Variables|Default|Getcount_score2) 1))
                                          (Variables|Default|Setcount_item2 (+ (Variables|Default|Getcount_item2) 1))
                                          (Variables|/Game/Blueprint/control/Mygame/MyGame.MyGame_C|Setlevel2_Yellow_Water-bottle2 (stale EventTick _asmy_game) (+ (Variables|/Game/Blueprint/control/Mygame/MyGame.MyGame_C|Getlevel2_Yellow_Water-bottle2 (stale EventTick _asmy_game)) 1))
                                          (Variables|/Game/Blueprint/control/Mygame/MyGame.MyGame_C|SetCheck_amount_item_Yellow2 (stale EventTick _asmy_game) (+ (Variables|/Game/Blueprint/control/Mygame/MyGame.MyGame_C|GetCheck_amount_item_Yellow2 (stale EventTick _asmy_game)) 1))
                                          (Audio|PlaySound2D "/Game/Map/sound/Wiget/correct.correct" 1.0 1.0 0.0 0 0))
                                        (:CastFailed
                                          ;[1 1 1] set hidden item and -score in count score (TBLUE) and count item
                                          (bind _asbp_candy (Utilities|Casting|CastToBP_Candy OtherActor)
                                            (:then
                                              (Actor|DestroyActor _asbp_candy)
                                              (Variables|Default|Setcount_score2 (- (Variables|Default|Getcount_score2) 1))
                                              (Variables|Default|Setcount_item2 (+ (Variables|Default|Getcount_item2) 1))
                                              ;;[1 1 1] check wrong item
                                              (Variables|/Game/Blueprint/control/Mygame/MyGame.MyGame_C|Setlevel2_Blue_Candy_check (stale EventTick _asmy_game) (+ (Variables|/Game/Blueprint/control/Mygame/MyGame.MyGame_C|Getlevel2_Blue_Candy_check (stale EventTick _asmy_game)) 2))
                                              (Audio|PlaySound2D "/Game/Map/sound/Wiget/wrong2.wrong2" 6.0 1.0 0.0 0 0))
                                            (:CastFailed
                                              (bind _asbp_jelly__bag (Utilities|Casting|CastToBP_Jelly-Bag OtherActor)
                                                (:then
                                                  (Actor|DestroyActor _asbp_jelly__bag)
                                                  (Variables|Default|Setcount_score2 (- (Variables|Default|Getcount_score2) 1))
                                                  (Variables|Default|Setcount_item2 (+ (Variables|Default|Getcount_item2) 1))
                                                  (Variables|/Game/Blueprint/control/Mygame/MyGame.MyGame_C|Setlevel2_Blue_Jelly-Bag_check (stale EventTick _asmy_game) (+ (Variables|/Game/Blueprint/control/Mygame/MyGame.MyGame_C|Getlevel2_Blue_Jelly-Bag_check (stale EventTick _asmy_game)) 2))
                                                  (Audio|PlaySound2D "/Game/Map/sound/Wiget/wrong2.wrong2" 6.0 1.0 0.0 0 0))
                                                (:CastFailed
                                                  (bind _asbp_plastic__bag (Utilities|Casting|CastToBP_Plastic-Bag OtherActor)
                                                    (:then
                                                      (Actor|DestroyActor _asbp_plastic__bag)
                                                      (Variables|Default|Setcount_score2 (- (Variables|Default|Getcount_score2) 1))
                                                      (Variables|Default|Setcount_item2 (+ (Variables|Default|Getcount_item2) 1))
                                                      (Variables|/Game/Blueprint/control/Mygame/MyGame.MyGame_C|Setlevel2_Blue_Plastic-Bag_check (stale EventTick _asmy_game) (+ (Variables|/Game/Blueprint/control/Mygame/MyGame.MyGame_C|Getlevel2_Blue_Plastic-Bag_check (stale EventTick _asmy_game)) 2))
                                                      (Audio|PlaySound2D "/Game/Map/sound/Wiget/wrong2.wrong2" 6.0 1.0 0.0 0 0))
                                                    (:CastFailed
                                                      (bind _asbp_snack__box (Utilities|Casting|CastToBP_Snack-Box OtherActor)
                                                        (:then
                                                          (Actor|DestroyActor _asbp_snack__box)
                                                          (Variables|Default|Setcount_score2 (- (Variables|Default|Getcount_score2) 1))
                                                          (Variables|Default|Setcount_item2 (+ (Variables|Default|Getcount_item2) 1))
                                                          (Variables|/Game/Blueprint/control/Mygame/MyGame.MyGame_C|Setlevel2_Blue_Snack-Box_check (stale EventTick _asmy_game) (+ (Variables|/Game/Blueprint/control/Mygame/MyGame.MyGame_C|Getlevel2_Blue_Snack-Box_check (stale EventTick _asmy_game)) 2))
                                                          (Audio|PlaySound2D "/Game/Map/sound/Wiget/wrong2.wrong2" 6.0 1.0 0.0 0 0))
                                                        (:CastFailed
                                                          (bind _asbp_toilet__paper (Utilities|Casting|CastToBP_Toilet-Paper OtherActor))
                                                          (Actor|DestroyActor _asbp_toilet__paper)
                                                          (Variables|Default|Setcount_score2 (- (Variables|Default|Getcount_score2) 1))
                                                          (Variables|Default|Setcount_item2 (+ (Variables|Default|Getcount_item2) 1))
                                                          (Variables|/Game/Blueprint/control/Mygame/MyGame.MyGame_C|Setlevel2_Blue_Toilet-Paper_check (stale EventTick _asmy_game) (+ (Variables|/Game/Blueprint/control/Mygame/MyGame.MyGame_C|Getlevel2_Blue_Toilet-Paper_check (stale EventTick _asmy_game)) 2))
                                                          (Audio|PlaySound2D "/Game/Map/sound/Wiget/wrong2.wrong2" 6.0 1.0 0.0 0 0))))))))))))))))))))))))))))))

(event EventBeginPlay)

(event EventTick
  (params (DeltaSeconds :type Float%20%28single-precision%29))
  ;[1 1 1] send score to mygame instant
  (bind _asmy_game (Utilities|Casting|CastToMyGame (Game|GetGameInstance)))
  (Variables|/Game/Blueprint/control/Mygame/MyGame.MyGame_C|Setscore_yellow2 _asmy_game (Variables|Default|Getcount_score2))
  (Variables|/Game/Blueprint/control/Mygame/MyGame.MyGame_C|Setcount_Allitem_yellow2 _asmy_game (Variables|Default|Getcount_item2)))

(fn ConstructionScript)