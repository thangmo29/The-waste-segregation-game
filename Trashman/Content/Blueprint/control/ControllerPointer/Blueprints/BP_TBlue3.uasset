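; Blue bin for level 3 of a waste-sorting game that scores items dropped into it.
; Sphere overlap runs a cast chain over item classes, destroys the match, counts it and adjusts score up for blue items, down for green, yellow or red ones.
; It also updates per-item MyGame counters and plays a correct or wrong sound, except for smartphones, which are silent.
; Tick casts the GameInstance to MyGame and copies score and item count into it.
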(event OnComponentBeginOverlap(Sphere)
  (params (OverlappedComponent :type Primitive%20Component%20Object%20Reference) (OtherActor :type Actor%20Object%20Reference) (OtherComp :type Primitive%20Component%20Object%20Reference) (OtherBodyIndex :type Integer) (bFromSweep :type Boolean) (SweepResult :type Hit%20Result%20Structure%20%28by%20ref%29))
  ;[1 1 1] set hidden item and -score in count_score (TGreen) and count item
  (bind _asbp_big_mac (Utilities|Casting|CastToBP_big-mac OtherActor)
    (:then
      (Actor|DestroyActor _asbp_big_mac)
      (Variables|Default|Setcount_score3 (- (Variables|Default|Getcount_score3) 1))
      ;;[1 1 1] check wrong item
      (Variables|Default|Setcount_item3 (+ (Variables|Default|Getcount_item3) 1))
      (Variables|/Game/Blueprint/control/Mygame/MyGame.MyGame_C|Setlevel3_Green_Hamburger_check (stale EventTick _asmy_game) (+ (Variables|/Game/Blueprint/control/Mygame/MyGame.MyGame_C|Getlevel3_Green_Hamburger_check (stale EventTick _asmy_game)) 3))
      (Audio|PlaySound2D "/Game/Map/sound/Wiget/wrong2.wrong2" 6.0 1.0 0.0 0 0))
    (:CastFailed
      (bind _asbp_chicken_leg (Utilities|Casting|CastToBP_chicken-leg OtherActor)
        (:then
          (Actor|DestroyActor _asbp_chicken_leg)
          (Variables|Default|Setcount_score3 (- (Variables|Default|Getcount_score3) 1))
          (Variables|Default|Setcount_item3 (+ (Variables|Default|Getcount_item3) 1))
          (Variables|/Game/Blueprint/control/Mygame/MyGame.MyGame_C|Setlevel3_Green_Chicken-Leg_check (stale EventTick _asmy_game) (+ (Variables|/Game/Blueprint/control/Mygame/MyGame.MyGame_C|Getlevel3_Green_Chicken-Leg_check (stale EventTick _asmy_game)) 3))
          (Audio|PlaySound2D "/Game/Map/sound/Wiget/wrong2.wrong2" 6.0 1.0 0.0 0 0))
        (:CastFailed
          (bind _asbp_elbsandsteinpilze (Utilities|Casting|CastToBP_elbsandsteinpilze OtherActor)
            (:then
              (Actor|DestroyActor _asbp_elbsandsteinpilze)
              (Variables|Default|Setcount_score3 (- (Variables|Default|Getcount_score3) 1))
              (Variables|Default|Setcount_item3 (+ (Variables|Default|Getcount_item3) 1))
              (Variables|/Game/Blueprint/control/Mygame/MyGame.MyGame_C|Setlevel3_Green_Food-Scrops_check (stale EventTick _asmy_game) (+ (Variables|/Game/Blueprint/control/Mygame/MyGame.MyGame_C|Getlevel3_Green_Food-Scrops_check (stale EventTick _asmy_game)) 3))
              (Audio|PlaySound2D "/Game/Map/sound/Wiget/wrong2.wrong2" 6.0 1.0 0.0 0 0))
            (:CastFailed
              (bind _asbp_fruit_aple (Utilities|Casting|CastToBP_fruit-aple OtherActor)
                (:then
                  (Actor|DestroyActor _asbp_fruit_aple)
                  (Variables|Default|Setcount_score3 (- (Variables|Default|Getcount_score3) 1))
                  (Variables|Default|Setcount_item3 (+ (Variables|Default|Getcount_item3) 1))
                  (Variables|/Game/Blueprint/control/Mygame/MyGame.MyGame_C|Setlevel3_Green_Apple_check (stale EventTick _asmy_game) (+ (Variables|/Game/Blueprint/control/Mygame/MyGame.MyGame_C|Getlevel3_Green_Apple_check (stale EventTick _asmy_game)) 3))
                  (Audio|PlaySound2D "/Game/Map/sound/Wiget/wrong2.wrong2" 6.0 1.0 0.0 0 0))
                (:CastFailed
                  (bind _asbp_pork_chop (Utilities|Casting|CastToBP_pork-chop OtherActor)
                    (:then
                      (Actor|DestroyActor _asbp_pork_chop)
                      (Variables|Default|Setcount_score3 (- (Variables|Default|Getcount_score3) 1))
                      (Variables|Default|Setcount_item3 (+ (Variables|Default|Getcount_item3) 1))
                      (Variables|/Game/Blueprint/control/Mygame/MyGame.MyGame_C|Setlevel3_Green_Pork-Chop_check (stale EventTick _asmy_game) (+ (Variables|/Game/Blueprint/control/Mygame/MyGame.MyGame_C|Getlevel3_Green_Pork-Chop_check (stale EventTick _asmy_game)) 3))
                      (Audio|PlaySound2D "/Game/Map/sound/Wiget/wrong2.wrong2" 6.0 1.0 0.0 0 0))
                    (:CastFailed
                      ;[1 1 1] set hidden item and -score in count_score (TYellow) and count item
                      (bind _asbp_beer_can (Utilities|Casting|CastToBP_beer-can OtherActor)
                        (:then
                          (Actor|DestroyActor _asbp_beer_can)
                          (Variables|Default|Setcount_score3 (- (Variables|Default|Getcount_score3) 1))
                          (Variables|Default|Setcount_item3 (+ (Variables|Default|Getcount_item3) 1))
                          ;;[1 1 1] check wrong item
                          (Variables|/Game/Blueprint/control/Mygame/MyGame.MyGame_C|Setlevel3_Yellow_Beer-Can_check (stale EventTick _asmy_game) (+ (Variables|/Game/Blueprint/control/Mygame/MyGame.MyGame_C|Getlevel3_Yellow_Beer-Can_check (stale EventTick _asmy_game)) 3))
                          (Audio|PlaySound2D "/Game/Map/sound/Wiget/wrong2.wrong2" 6.0 1.0 0.0 0 0))
                        (:CastFailed
                          (bind _asbp_cardboard_box (Utilities|Casting|CastToBP_cardboard-box OtherActor)
                            (:then
                              (Actor|DestroyActor _asbp_cardboard_box)
                              (Variables|Default|Setcount_score3 (- (Variables|Default|Getcount_score3) 1))
                              (Variables|Default|Setcount_item3 (+ (Variables|Default|Getcount_item3) 1))
                              (Variables|/Game/Blueprint/control/Mygame/MyGame.MyGame_C|Setlevel3_Yellow_Cardboard-Box_check (stale EventTick _asmy_game) (+ (Variables|/Game/Blueprint/control/Mygame/MyGame.MyGame_C|Getlevel3_Yellow_Cardboard-Box_check (stale EventTick _asmy_game)) 3))
                              (Audio|PlaySound2D "/Game/Map/sound/Wiget/wrong2.wrong2" 6.0 1.0 0.0 0 0))
                            (:CastFailed
                              (bind _asbp_cola_can (Utilities|Casting|CastToBP_cola-can OtherActor)
                                (:then
                                  (Actor|DestroyActor _asbp_cola_can)
                                  (Variables|Default|Setcount_score3 (- (Variables|Default|Getcount_score3) 1))
                                  (Variables|Default|Setcount_item3 (+ (Variables|Default|Getcount_item3) 1))
                                  (Variables|/Game/Blueprint/control/Mygame/MyGame.MyGame_C|Setlevel3_Yellow_Cola-Can_check (stale EventTick _asmy_game) (+ (Variables|/Game/Blueprint/control/Mygame/MyGame.MyGame_C|Getlevel3_Yellow_Cola-Can_check (stale EventTick _asmy_game)) 3))
                                  (Audio|PlaySound2D "/Game/Map/sound/Wiget/wrong2.wrong2" 6.0 1.0 0.0 0 0))
                                (:CastFailed
                                  (bind _asbp_monkey_bottle (Utilities|Casting|CastToBP_monkey-bottle OtherActor)
                                    (:then
                                      (Actor|DestroyActor _asbp_monkey_bottle)
                                      (Variables|Default|Setcount_score3 (- (Variables|Default|Getcount_score3) 1))
                                      (Variables|Default|Setcount_item3 (+ (Variables|Default|Getcount_item3) 1))
                                      (Variables|/Game/Blueprint/control/Mygame/MyGame.MyGame_C|Setlevel3_Yellow_Vodka-Bottle_check (stale EventTick _asmy_game) (+ (Variables|/Game/Blueprint/control/Mygame/MyGame.MyGame_C|Getlevel3_Yellow_Vodka-Bottle_check (stale EventTick _asmy_game)) 3))
                                      (Audio|PlaySound2D "/Game/Map/sound/Wiget/wrong2.wrong2" 6.0 1.0 0.0 0 0))
                                    (:CastFailed
                                      (bind _asbp_water_bottle (Utilities|Casting|CastToBP_water-bottle OtherActor)
                                        (:then
                                          (Actor|DestroyActor _asbp_water_bottle)
                                          (Variables|Default|Setcount_score3 (- (Variables|Default|Getcount_score3) 1))
                                          (Variables|Default|Setcount_item3 (+ (Variables|Default|Getcount_item3) 1))
                                          (Variables|/Game/Blueprint/control/Mygame/MyGame.MyGame_C|Setlevel3_Yellow_Water-Bottle_check (stale EventTick _asmy_game) (+ (Variables|/Game/Blueprint/control/Mygame/MyGame.MyGame_C|Getlevel3_Yellow_Water-Bottle_check (stale EventTick _asmy_game)) 3))
                                          (Audio|PlaySound2D "/Game/Map/sound/Wiget/wrong2.wrong2" 6.0 1.0 0.0 0 0))
                                        (:CastFailed
                                          ;[1 1 1] set hidden item and +score in count score (TBLUE) and count item
                                          (bind _asbp_almonds_snack (Utilities|Casting|CastToBP_almonds-snack OtherActor)
                                            (:then
                                              (Actor|DestroyActor _asbp_almonds_snack)
                                              (Variables|Default|Setcount_score3 (+ (Variables|Default|Getcount_score3) 1))
                                              (Variables|Default|Setcount_item3 (+ (Variables|Default|Getcount_item3) 1))
                                              (Variables|/Game/Blueprint/control/Mygame/MyGame.MyGame_C|Setlevel3_Blue_Almonds-Snack (stale EventTick _asmy_game) (+ (Variables|/Game/Blueprint/control/Mygame/MyGame.MyGame_C|Getlevel3_Blue_Almonds-Snack (stale EventTick _asmy_game)) 1))
                                              (Variables|/Game/Blueprint/control/Mygame/MyGame.MyGame_C|SetCheck_amount_item_Blue3 (stale EventTick _asmy_game) (+ (Variables|/Game/Blueprint/control/Mygame/MyGame.MyGame_C|GetCheck_amount_item_Blue3 (stale EventTick _asmy_game)) 1))
                                              (Audio|PlaySound2D "/Game/Map/sound/Wiget/correct.correct" 1.0 1.0 0.0 0 0))
                                            (:CastFailed
                                              (bind _asbp_burger_box (Utilities|Casting|CastToBP_burger-box OtherActor)
                                                (:then
                                                  (Actor|DestroyActor _asbp_burger_box)
                                                  (Variables|Default|Setcount_score3 (+ (Variables|Default|Getcount_score3) 1))
                                                  (Variables|Default|Setcount_item3 (+ (Variables|Default|Getcount_item3) 1))
                                                  (Variables|/Game/Blueprint/control/Mygame/MyGame.MyGame_C|Setlevel3_Blue_Burger-Box (stale EventTick _asmy_game) (+ (Variables|/Game/Blueprint/control/Mygame/MyGame.MyGame_C|Getlevel3_Blue_Burger-Box (stale EventTick _asmy_game)) 1))
                                                  (Variables|/Game/Blueprint/control/Mygame/MyGame.MyGame_C|SetCheck_amount_item_Blue3 (stale EventTick _asmy_game) (+ (Variables|/Game/Blueprint/control/Mygame/MyGame.MyGame_C|GetCheck_amount_item_Blue3 (stale EventTick _asmy_game)) 1))
                                                  (Audio|PlaySound2D "/Game/Map/sound/Wiget/correct.correct" 1.0 1.0 0.0 0 0))
                                                (:CastFailed
                                                  (bind _asbp_glove (Utilities|Casting|CastToBP_Glove OtherActor)
                                                    (:then
                                                      (Actor|DestroyActor _asbp_glove)
                                                      (Variables|Default|Setcount_score3 (+ (Variables|Default|Getcount_score3) 1))
                                                      (Variables|Default|Setcount_item3 (+ (Variables|Default|Getcount_item3) 1))
                                                      (Variables|/Game/Blueprint/control/Mygame/MyGame.MyGame_C|Setlevel3_Blue_Glove (stale EventTick _asmy_game) (+ (Variables|/Game/Blueprint/control/Mygame/MyGame.MyGame_C|Getlevel3_Blue_Glove (stale EventTick _asmy_game)) 1))
                                                      (Variables|/Game/Blueprint/control/Mygame/MyGame.MyGame_C|SetCheck_amount_item_Blue3 (stale EventTick _asmy_game) (+ (Variables|/Game/Blueprint/control/Mygame/MyGame.MyGame_C|GetCheck_amount_item_Blue3 (stale EventTick _asmy_game)) 1))
                                                      (Audio|PlaySound2D "/Game/Map/sound/Wiget/correct.correct" 1.0 1.0 0.0 0 0))
                                                    (:CastFailed
                                                      (bind _asbp_latex_gloves (Utilities|Casting|CastToBP_latex-gloves OtherActor)
                                                        (:then
                                                          (Actor|DestroyActor _asbp_latex_gloves)
                                                          (Variables|Default|Setcount_score3 (+ (Variables|Default|Getcount_score3) 1))
                                                          (Variables|Default|Setcount_item3 (+ (Variables|Default|Getcount_item3) 1))
                                                          (Variables|/Game/Blueprint/control/Mygame/MyGame.MyGame_C|Setlevel3_Blue_Gloves (stale EventTick _asmy_game) (+ (Variables|/Game/Blueprint/control/Mygame/MyGame.MyGame_C|Getlevel3_Blue_Gloves (stale EventTick _asmy_game)) 1))
                                                          (Variables|/Game/Blueprint/control/Mygame/MyGame.MyGame_C|SetCheck_amount_item_Blue3 (stale EventTick _asmy_game) (+ (Variables|/Game/Blueprint/control/Mygame/MyGame.MyGame_C|GetCheck_amount_item_Blue3 (stale EventTick _asmy_game)) 1))
                                                          (Audio|PlaySound2D "/Game/Map/sound/Wiget/correct.correct" 1.0 1.0 0.0 0 0))
                                                        (:CastFailed
                                                          (bind _asbp_potato_chips (Utilities|Casting|CastToBP_potato-chips OtherActor)
                                                            (:then
                                                              (Actor|DestroyActor _asbp_potato_chips)
                                                              (Variables|Default|Setcount_score3 (+ (Variables|Default|Getcount_score3) 1))
                                                              (Variables|Default|Setcount_item3 (+ (Variables|Default|Getcount_item3) 1))
                                                              (Variables|/Game/Blueprint/control/Mygame/MyGame.MyGame_C|Setlevel3_Blue_Potato-Chips (stale EventTick _asmy_game) (+ (Variables|/Game/Blueprint/control/Mygame/MyGame.MyGame_C|Getlevel3_Blue_Potato-Chips (stale EventTick _asmy_game)) 1))
                                                              (Variables|/Game/Blueprint/control/Mygame/MyGame.MyGame_C|SetCheck_amount_item_Blue3 (stale EventTick _asmy_game) (+ (Variables|/Game/Blueprint/control/Mygame/MyGame.MyGame_C|GetCheck_amount_item_Blue3 (stale EventTick _asmy_game)) 1))
                                                              (Audio|PlaySound2D "/Game/Map/sound/Wiget/correct.correct" 1.0 1.0 0.0 0 0))
                                                            (:CastFailed
                                                              ;[1 1 1] set hidden item and -score in count item (TRed) and count item
                                                              (bind _asbp_battery (Utilities|Casting|CastToBP_battery OtherActor)
                                                                (:then
                                                                  (Actor|DestroyActor _asbp_battery)
                                                                  (Variables|Default|Setcount_score3 (- (Variables|Default|Getcount_score3) 1))
                                                                  (Variables|Default|Setcount_item3 (+ (Variables|Default|Getcount_item3) 1))
                                                                  ;;[1 1 1] check wrong item
                                                                  (Variables|/Game/Blueprint/control/Mygame/MyGame.MyGame_C|Setlevel3_Red_Battery_check (stale EventTick _asmy_game) (+ (Variables|/Game/Blueprint/control/Mygame/MyGame.MyGame_C|Getlevel3_Red_Battery_check (stale EventTick _asmy_game)) 3))
                                                                  (Audio|PlaySound2D "/Game/Map/sound/Wiget/wrong2.wrong2" 6.0 1.0 0.0 0 0))
                                                                (:CastFailed
                                                                  (bind _asbp_light_bulb_kit (Utilities|Casting|CastToBP_light-bulb-kit OtherActor)
                                                                    (:then
                                                                      (Actor|DestroyActor _asbp_light_bulb_kit)
                                                                      (Variables|Default|Setcount_score3 (- (Variables|Default|Getcount_score3) 1))
                                                                      (Variables|Default|Setcount_item3 (+ (Variables|Default|Getcount_item3) 1))
                                                                      (Variables|/Game/Blueprint/control/Mygame/MyGame.MyGame_C|Setlevel3_Red_Light-Bulb_check (stale EventTick _asmy_game) (+ (Variables|/Game/Blueprint/control/Mygame/MyGame.MyGame_C|Getlevel3_Red_Light-Bulb_check (stale EventTick _asmy_game)) 3))
                                                                      (Audio|PlaySound2D "/Game/Map/sound/Wiget/wrong2.wrong2" 6.0 1.0 0.0 0 0))
                                                                    (:CastFailed
                                                                      (bind _asbp_face_mask (Utilities|Casting|CastToBP_face-mask OtherActor)
                                                                        (:then
                                                                          (Actor|DestroyActor _asbp_face_mask)
                                                                          (Variables|Default|Setcount_score3 (- (Variables|Default|Getcount_score3) 1))
                                                                          (Variables|Default|Setcount_item3 (+ (Variables|Default|Getcount_item3) 1))
                                                                          (Variables|/Game/Blueprint/control/Mygame/MyGame.MyGame_C|Setlevel3_Red_Face-Mask_check (stale EventTick _asmy_game) (+ (Variables|/Game/Blueprint/control/Mygame/MyGame.MyGame_C|Getlevel3_Red_Face-Mask_check (stale EventTick _asmy_game)) 3))
                                                                          (Audio|PlaySound2D "/Game/Map/sound/Wiget/wrong2.wrong2" 6.0 1.0 0.0 0 0))
                                                                        (:CastFailed
                                                                          (bind _asbp_smartphone (Utilities|Casting|CastToBP_smartphone OtherActor)
                                                                            (:then
                                                                              (Actor|DestroyActor _asbp_smartphone)
                                                                              (Variables|Default|Setcount_score3 (- (Variables|Default|Getcount_score3) 1))
                                                                              (Variables|Default|Setcount_item3 (+ (Variables|Default|Getcount_item3) 1))
                                                                              (Variables|/Game/Blueprint/control/Mygame/MyGame.MyGame_C|Setlevel3_Red_Smartphone_check (stale EventTick _asmy_game) (+ (Variables|/Game/Blueprint/control/Mygame/MyGame.MyGame_C|Getlevel3_Red_Smartphone_check (stale EventTick _asmy_game)) 3)))
                                                                            (:CastFailed
                                                                              (bind _asbp_spray_can (Utilities|Casting|CastToBP_spray-can OtherActor))
                                                                              (Actor|DestroyActor _asbp_spray_can)
                                                                              (Variables|Default|Setcount_score3 (- (Variables|Default|Getcount_score3) 1))
                                                                              (Variables|Default|Setcount_item3 (+ (Variables|Default|Getcount_item3) 1))
                                                                              (Variables|/Game/Blueprint/control/Mygame/MyGame.MyGame_C|Setlevel3_Red_Spray_check (stale EventTick _asmy_game) (+ (Variables|/Game/Blueprint/control/Mygame/MyGame.MyGame_C|Getlevel3_Red_Spray_check (stale EventTick _asmy_game)) 3))
                                                                              (Audio|PlaySound2D "/Game/Map/sound/Wiget/wrong2.wrong2" 6.0 1.0 0.0 0 0))))))))))))))))))))))))))))))))))))))))

(event EventBeginPlay)

(event EventTick
  (params (DeltaSeconds :type Float%20%28single-precision%29))
  ;[1 1 1] send score to mygame instant
  (bind _asmy_game (Utilities|Casting|CastToMyGame (Game|GetGameInstance)))
  (Variables|/Game/Blueprint/control/Mygame/MyGame.MyGame_C|Setscore_blue3 _asmy_game (Variables|Default|Getcount_score3))
  (Variables|/Game/Blueprint/control/Mygame/MyGame.MyGame_C|Setcount_Allitem_blue3 _asmy_game (Variables|Default|Getcount_item3)))

(fn ConstructionScript)