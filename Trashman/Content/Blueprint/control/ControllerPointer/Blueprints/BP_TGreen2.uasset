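; Green trash bin in a waste-sorting game that scores items dropped into it.
; Its sphere overlap runs a cast chain over item classes, destroying each match and counting it.
; Food waste adds a point with a correct sound, while items for the yellow and blue bins subtract one with a wrong sound.
; Tick copies the score and item count to the MyGame game instance every frame.
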(event OnComponentBeginOverlap(Sphere)
  (params (OverlappedComponent :type Primitive%20Component%20Object%20Reference) (OtherActor :type Actor%20Object%20Reference) (OtherComp :type Primitive%20Component%20Object%20Reference) (OtherBodyIndex :type Integer) (bFromSweep :type Boolean) (SweepResult :type Hit%20Result%20Structure%20%28by%20ref%29))
  ;[1 1 1] set hidden item and +score in count_score (TGreen) and count item
  (bind _asbp_banana (Utilities|Casting|CastToBP_Banana OtherActor)
    (:then
      (Actor|DestroyActor _asbp_banana)
      (Variables|Default|Setcount_score1 (+ (Variables|Default|Getcount_score1) 1))
      (Variables|Default|Setcount_item1 (+ (Variables|Default|Getcount_item1) 1))
      (Audio|PlaySound2D "/Game/Map/sound/Wiget/correct.correct" 1.0 1.0 0.0 0 0))
    (:CastFailed
      (bind _asbp_hotdog (Utilities|Casting|CastToBP_Hotdog OtherActor)
        (:then
          (Actor|DestroyActor _asbp_hotdog)
          (Variables|Default|Setcount_score1 (+ (Variables|Default|Getcount_score1) 1))
          (Variables|Default|Setcount_item1 (+ (Variables|Default|Getcount_item1) 1))
          (Audio|PlaySound2D "/Game/Map/sound/Wiget/correct.correct" 1.0 1.0 0.0 0 0))
        (:CastFailed
          (bind _asbp_orange (Utilities|Casting|CastToBP_Orange OtherActor)
            (:then
              (Actor|DestroyActor _asbp_orange)
              (Variables|Default|Setcount_score1 (+ (Variables|Default|Getcount_score1) 1))
              (Variables|Default|Setcount_item1 (+ (Variables|Default|Getcount_item1) 1))
              (Audio|PlaySound2D "/Game/Map/sound/Wiget/correct.correct" 1.0 1.0 0.0 0 0))
            (:CastFailed
              (bind _asbp_pig__bone (Utilities|Casting|CastToBP_Pig-Bone OtherActor)
                (:then
                  (Actor|DestroyActor _asbp_pig__bone)
                  (Variables|Default|Setcount_score1 (+ (Variables|Default|Getcount_score1) 1))
                  (Variables|Default|Setcount_item1 (+ (Variables|Default|Getcount_item1) 1))
                  (Audio|PlaySound2D "/Game/Map/sound/Wiget/correct.correct" 1.0 1.0 0.0 0 0))
                (:CastFailed
                  (bind _asbp_strawberry (Utilities|Casting|CastToBP_Strawberry OtherActor)
                    (:then
                      (Actor|DestroyActor _asbp_strawberry)
                      (Variables|Default|Setcount_score1 (+ (Variables|Default|Getcount_score1) 1))
                      (Variables|Default|Setcount_item1 (+ (Variables|Default|Getcount_item1) 1))
                      (Audio|PlaySound2D "/Game/Map/sound/Wiget/correct.correct" 1.0 1.0 0.0 0 0))
                    (:CastFailed
                      ;[1 1 1] set hidden item and -score in count_score (TYellow) and count item
                      (bind _asbp_can (Utilities|Casting|CastToBP_Can OtherActor)
                        (:then
                          (Actor|DestroyActor _asbp_can)
                          (Variables|Default|Setcount_score1 (- (Variables|Default|Getcount_score1) 1))
                          (Variables|Default|Setcount_item1 (+ (Variables|Default|Getcount_item1) 1))
                          (Audio|PlaySound2D "/Game/Map/sound/Wiget/wrong2.wrong2" 6.0 1.0 0.0 0 0))
                        (:CastFailed
                          (bind _asbp_cardboard_box_2 (Utilities|Casting|CastToBP_Cardboard-box2 OtherActor)
                            (:then
                              (Actor|DestroyActor _asbp_cardboard_box_2)
                              (Variables|Default|Setcount_score1 (- (Variables|Default|Getcount_score1) 1))
                              (Variables|Default|Setcount_item1 (+ (Variables|Default|Getcount_item1) 1))
                              (Audio|PlaySound2D "/Game/Map/sound/Wiget/wrong2.wrong2" 6.0 1.0 0.0 0 0))
                            (:CastFailed
                              (bind _asbp_milk__box (Utilities|Casting|CastToBP_Milk-Box OtherActor)
                                (:then
                                  (Actor|DestroyActor _asbp_milk__box)
                                  (Variables|Default|Setcount_score1 (- (Variables|Default|Getcount_score1) 1))
                                  (Variables|Default|Setcount_item1 (+ (Variables|Default|Getcount_item1) 1))
                                  (Audio|PlaySound2D "/Game/Map/sound/Wiget/wrong2.wrong2" 6.0 1.0 0.0 0 0))
                                (:CastFailed
                                  (bind _asbp_soup_can (Utilities|Casting|CastToBP_Soup-can OtherActor)
                                    (:then
                                      (Actor|DestroyActor _asbp_soup_can)
                                      (Variables|Default|Setcount_score1 (- (Variables|Default|Getcount_score1) 1))
                                      (Variables|Default|Setcount_item1 (+ (Variables|Default|Getcount_item1) 1))
                                      (Audio|PlaySound2D "/Game/Map/sound/Wiget/wrong2.wrong2" 6.0 1.0 0.0 0 0))
                                    (:CastFailed
                                      (bind _asbp_water_bottle_2 (Utilities|Casting|CastToBP_Water-bottle2 OtherActor)
                                        (:then
                                          (Actor|DestroyActor _asbp_water_bottle_2)
                                          (Variables|Default|Setcount_score1 (- (Variables|Default|Getcount_score1) 1))
                                          (Variables|Default|Setcount_item1 (+ (Variables|Default|Getcount_item1) 1))
                                          (Audio|PlaySound2D "/Game/Map/sound/Wiget/wrong2.wrong2" 6.0 1.0 0.0 0 0))
                                        (:CastFailed
                                          ;[1 1 1] set hidden item and -score in count score (TBLUE) and count item
                                          (bind _asbp_candy (Utilities|Casting|CastToBP_Candy OtherActor)
                                            (:then
                                              (Actor|DestroyActor _asbp_candy)
                                              (Variables|Default|Setcount_score1 (- (Variables|Default|Getcount_score1) 1))
                                              (Variables|Default|Setcount_item1 (+ (Variables|Default|Getcount_item1) 1))
                                              (Audio|PlaySound2D "/Game/Map/sound/Wiget/wrong2.wrong2" 6.0 1.0 0.0 0 0))
                                            (:CastFailed
                                              (bind _asbp_jenny__bag (Utilities|Casting|CastToBP_Jenny-Bag OtherActor)
                                                (:then
                                                  (Actor|DestroyActor _asbp_jenny__bag)
                                                  (Variables|Default|Setcount_score1 (- (Variables|Default|Getcount_score1) 1))
                                                  (Variables|Default|Setcount_item1 (+ (Variables|Default|Getcount_item1) 1))
                                                  (Audio|PlaySound2D "/Game/Map/sound/Wiget/wrong2.wrong2" 6.0 1.0 0.0 0 0))
                                                (:CastFailed
                                                  (bind _asbp_plastic__bag (Utilities|Casting|CastToBP_Plastic-Bag OtherActor)
                                                    (:then
                                                      (Actor|DestroyActor _asbp_plastic__bag)
                                                      (Variables|Default|Setcount_score1 (- (Variables|Default|Getcount_score1) 1))
                                                      (Variables|Default|Setcount_item1 (+ (Variables|Default|Getcount_item1) 1))
                                                      (Audio|PlaySound2D "/Game/Map/sound/Wiget/wrong2.wrong2" 6.0 1.0 0.0 0 0))
                                                    (:CastFailed
                                                      (bind _asbp_snack__box (Utilities|Casting|CastToBP_Snack-Box OtherActor)
                                                        (:then
                                                          (Actor|DestroyActor _asbp_snack__box)
                                                          (Variables|Default|Setcount_score1 (- (Variables|Default|Getcount_score1) 1))
                                                          (Variables|Default|Setcount_item1 (+ (Variables|Default|Getcount_item1) 1))
                                                          (Audio|PlaySound2D "/Game/Map/sound/Wiget/wrong2.wrong2" 6.0 1.0 0.0 0 0))
                                                        (:CastFailed
                                                          (bind _asbp_toilet__paper (Utilities|Casting|CastToBP_Toilet-Paper OtherActor))
                                                          (Actor|DestroyActor _asbp_toilet__paper)
                                                          (Variables|Default|Setcount_score1 (- (Variables|Default|Getcount_score1) 1))
                                                          (Variables|Default|Setcount_item1 (+ (Variables|Default|Getcount_item1) 1))
                                                          (Audio|PlaySound2D "/Game/Map/sound/Wiget/wrong2.wrong2" 6.0 1.0 0.0 0 0))))))))))))))))))))))))))))))

(event EventBeginPlay)

(event Collision|EventActorBeginOverlap
  (params (OtherActor :type Actor%20Object%20Reference)))

(event EventTick
  (params (DeltaSeconds :type Float%20%28single-precision%29))
  ;[1 1 1] send score to mygame instant
  (bind _asmy_game (Utilities|Casting|CastToMyGame (Game|GetGameInstance)))
  (Variables|/Game/Blueprint/control/Mygame/MyGame.MyGame_C|Setscore_green2 _asmy_game (Variables|Default|Getcount_score1))
  (Variables|/Game/Blueprint/control/Mygame/MyGame.MyGame_C|Setcount_Allitem_green2 _asmy_game (Variables|Default|Getcount_item1)))

(fn ConstructionScript)