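; BP_TGreen is a scoring target, apparently the green bin in a waste-sorting game, that destroys item actors overlapping its sphere.
; A cast chain identifies each item: food raises CountScore1, while cans, bottles and cardboard lower it.
; The big-mac branch differs by incrementing the game instance's ScoreCount1 and copying the result into CountScore1.
; Tick casts to the MyGame instance and writes CountScore1 to ScoreGreen1 every frame.
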(event OnComponentBeginOverlap(Sphere)
  (params (OverlappedComponent :type Primitive%20Component%20Object%20Reference) (OtherActor :type Actor%20Object%20Reference) (OtherComp :type Primitive%20Component%20Object%20Reference) (OtherBodyIndex :type Integer) (bFromSweep :type Boolean) (SweepResult :type Hit%20Result%20Structure%20%28by%20ref%29))
  ;[1 1 1] set hidden item and +score in count_score (TGreen)
  (bind _asbp_big_mac (Utilities|Casting|CastToBP_big-mac OtherActor)
    (:then
      (Actor|DestroyActor _asbp_big_mac)
      (bind _result (Math|Integer|IncrementInt (Variables|/Game/Blueprint/control/Mygame/MyGame.MyGame_C|Getscore_count1 (stale EventTick _asmy_game)))
        (:%20%20
          (bind _output_get (Variables|Default|Setcount_score1 _result)))))
    (:CastFailed
      _))
  (bind _asbp_chicken_leg (Utilities|Casting|CastToBP_chicken-leg OtherActor)
    (:then
      (Actor|DestroyActor _asbp_chicken_leg)
      (bind _result_2 (Math|Integer|IncrementInt _output_get)
        (:%20%20
          (bind _output_get_2 (Variables|Default|Setcount_score1 _result_2)))))
    (:CastFailed
      (bind _asbp_elbsandsteinpilze (Utilities|Casting|CastToBP_elbsandsteinpilze OtherActor)
        (:then
          (Actor|DestroyActor _asbp_elbsandsteinpilze)
          (bind _result_3 (Math|Integer|IncrementInt _output_get_2)
            (:%20%20
              (bind _output_get_3 (Variables|Default|Setcount_score1 _result_3)))))
        (:CastFailed
          (bind _asbp_fruit_aple (Utilities|Casting|CastToBP_fruit-aple OtherActor)
            (:then
              (Actor|DestroyActor _asbp_fruit_aple)
              (bind _result_4 (Math|Integer|IncrementInt _output_get_3)
                (:%20%20
                  (bind _output_get_4 (Variables|Default|Setcount_score1 _result_4)))))
            (:CastFailed
              (bind _asbp_pork_chop (Utilities|Casting|CastToBP_pork-chop OtherActor)
                (:then
                  (Actor|DestroyActor _asbp_pork_chop)
                  (bind _result_5 (Math|Integer|IncrementInt _output_get_4)
                    (:%20%20
                      (bind _output_get_5 (Variables|Default|Setcount_score1 _result_5)))))
                (:CastFailed
                  ;[1 1 1] set hidden item and -score in count_score (TYellow)
                  (bind _asbp_beer_can (Utilities|Casting|CastToBP_beer-can OtherActor)
                    (:then
                      (Actor|DestroyActor _asbp_beer_can)
                      (bind _result_6 (Math|Integer|DecrementInt _output_get_5)
                        (:%20%20
                          (bind _output_get_6 (Variables|Default|Setcount_score1 _result_6)))))
                    (:CastFailed
                      (bind _asbp_cardboard_box (Utilities|Casting|CastToBP_cardboard-box OtherActor)
                        (:then
                          (Actor|DestroyActor _asbp_cardboard_box)
                          (bind _result_7 (Math|Integer|DecrementInt _output_get_6)
                            (:%20%20
                              (bind _output_get_7 (Variables|Default|Setcount_score1 _result_7)))))
                        (:CastFailed
                          (bind _asbp_cola_can (Utilities|Casting|CastToBP_cola-can OtherActor)
                            (:then
                              (Actor|DestroyActor _asbp_cola_can)
                              (bind _result_8 (Math|Integer|DecrementInt _output_get_7)
                                (:%20%20
                                  (bind _output_get_8 (Variables|Default|Setcount_score1 _result_8)))))
                            (:CastFailed
                              (bind _asbp_monkey_bottle (Utilities|Casting|CastToBP_monkey-bottle OtherActor)
                                (:then
                                  (Actor|DestroyActor _asbp_monkey_bottle)
                                  (bind _result_9 (Math|Integer|DecrementInt _output_get_8)
                                    (:%20%20
                                      (bind _output_get_9 (Variables|Default|Setcount_score1 _result_9)))))
                                (:CastFailed
                                  (bind _asbp_water_bottle (Utilities|Casting|CastToBP_water-bottle OtherActor))
                                  (Actor|DestroyActor _asbp_water_bottle)
                                  (bind _result_10 (Math|Integer|DecrementInt _output_get_9)
                                    (:%20%20
                                      (Variables|Default|Setcount_score1 _result_10))))))))))))))))))))

(event EventBeginPlay)

(event Collision|EventActorBeginOverlap
  (params (OtherActor :type Actor%20Object%20Reference)))

(event EventTick
  (params (DeltaSeconds :type Float%20%28single-precision%29))
  ;[1 1 1] send score to mygame instant
  (bind _asmy_game (Utilities|Casting|CastToMyGame (Game|GetGameInstance)))
  (Variables|/Game/Blueprint/control/Mygame/MyGame.MyGame_C|Setscore_green1 _asmy_game (Variables|Default|Getcount_score1)))

(fn ConstructionScript)