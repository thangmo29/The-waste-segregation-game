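; Places a hidden Content actor on the floor where the XR user looks, then opens the Home level.
; It attaches to the XR pawn's camera so prompt text follows, while a looping timer line-traces forward from the camera.
; Placement requires a time counter near TimeToPlace, matching pre- and post-trace camera transforms, and a grid-snapped upward hit normal.
; On success it detaches, reveals and moves Content, stops tracing and removes the text.
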(event Custom|requestRaycast
  (bind _returnvalue (Game|GetPlayerCameraManager 0))
  (bind _transformcomponent (Variables|/Script/Engine.PlayerCameraManager|GetTransformComponent _returnvalue))
  (bind _returnvalue_2 (Transformation|GetWorldLocation _transformcomponent))
  ;[1 1 1] Toggle raycast based on looping bool
  (if (Variables|Default|Getlooping)
    ;[1 1 1] capture camera transform before raycast
    (Variables|Default|SetCameraTransform (Transformation|GetWorldTransform _transformcomponent))
    ;[1 1 1] Raycast
    (bind (_outhit _returnvalue_3) (Collision|LineTraceByChannel _returnvalue_2 (+ _returnvalue_2 (* (Math|Vector|Normalize (Math|Vector|GetForwardVector _transformcomponent)) 5e+02)) "TraceTypeQuery1" false 0 "None"))
    (if _returnvalue_3 ; Did the raycast hit something
      ;[1 1 1] GameTime counter
      (bind _output_get (Variables|Default|SetCount (+ (stale EventTick DeltaSeconds) (Variables|Default|GetCount))))
      (if (Math|Boolean|ANDBoolean (Math|Float|NearlyEqual(Float) _output_get (Variables|Default|GetTimeToPlace) 0.1) (Class|KismetMathLibrary|NearlyEqualTransformTransform (Transformation|GetWorldTransform (Variables|/Script/Engine.PlayerCameraManager|GetTransformComponent (Game|GetPlayerCameraManager 0))) (Variables|Default|GetCameraTransform) 1.0 1.0 1.0) (== (Math|Float|SnapToGrid(Float) (.pitch (Math|Conversions|RotationFromXVector (.ImpactNormal (Collision|BreakHitResult _outhit)))) 9e+01) 9e+01)) ; Did we hit all 3 conditions?
        ;[1 1 1] Unhide static mesh, detach from actor and move static mesh to raycast hit location
        (Development|SetHiddeninGame (Variables|/Script/Engine.Actor|GetRootComponent (Variables|Default|GetContent)) false true)
        (Transformation|DetachFromActor "KeepRelative" "KeepRelative" "KeepRelative")
        (Transformation|SetActorLocationAndRotation (Variables|Default|GetContent) (.Location (Collision|BreakHitResult _outhit)) (Math|Rotator|MakeRotator (.roll (Math|Conversions|RotationFromXVector (.ImpactNormal (Collision|BreakHitResult _outhit)))) (Math|Float|SnapToGrid(Float) (.pitch (Math|Conversions|RotationFromXVector (.ImpactNormal (Collision|BreakHitResult _outhit)))) 9e+01) (.yaw (Math|Conversions|RotationFromXVector (.ImpactNormal (Collision|BreakHitResult _outhit))))))
        (Variables|Default|Setlooping false) ; End Loop for Raycast
        (Game|OpenLevel(byName) "Home")
        (Components|DestroyComponent (Variables|Default|GetTextRender)) ; Remove text
        (elif (>= (Variables|Default|GetCount) (Variables|Default|GetTimeToPlace)) ; Did we fail previous check due to time?
          (Variables|Default|SetCount 0.0))))))

(event EventBeginPlay
  ;[1 1 1] Get XRPawn from Level. Attach to the camera to allow text to follow
  (bind _outactors (Actor|GetAllActorsOfClass "/Game/Blueprint/control/Common/BP_XRPawn.BP_XRPawn_C"))
  (bind _output_get (Variables|Default|SetXRPawn (Utilities|Array|Get(acopy) _outactors)))
  (Transformation|AttachComponentToComponent (Variables|/Game/Blueprint/control/Common/BP_XRPawn.BP_XRPawn_C|GetXR_Camera _output_get) "None" "KeepRelative" "KeepRelative" "KeepRelative" true)
  (Development|SetHiddeninGame (Variables|/Script/Engine.Actor|GetRootComponent (Variables|Default|GetContent)) true false) ; Verify that the static mesh is hidden at launch
  (Utilities|Time|SetTimerbyEvent (delegate Custom|requestRaycast) 0.1 true))

(event Collision|EventActorBeginOverlap
  (params (OtherActor :type Actor%20Object%20Reference)))

(event EventTick
  (params (DeltaSeconds :type Float%20%28single-precision%29))
  ;[1 1 1] GameTime counter
)

(fn ConstructionScript
  (Rendering|SetActorHiddenInGame (Variables|Default|GetContent) true))