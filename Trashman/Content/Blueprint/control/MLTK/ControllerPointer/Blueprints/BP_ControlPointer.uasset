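; Magic Leap controller laser pointer that attaches to the XR pawn's motion controller to highlight, grab and manipulate objects.
; Each tick it line-traces from the controller, tints the hit component and bends a spline-mesh beam to it.
; Holding the trigger grabs via a PhysicsHandle, while touchpad gestures scale, push/pull and yaw the object until release restores its scale.
; Reaching the arm out from the headset lengthens the ray and extends the held object's target.
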(event EventBeginPlay
  (bind _outactors (Actor|GetAllActorsOfClass "/Game/Blueprint/control/MLTK/Common/BP_XRPawn.BP_XRPawn_C"))
  (bind _output_get (Variables|Default|SetXRPawn (Utilities|Array|Get(acopy) _outactors)))
  (Input|EnableInput (Game|GetPlayerController 0))
  (Transformation|AttachComponentToComponent (Variables|/Game/Blueprint/control/MLTK/Common/BP_XRPawn.BP_XRPawn_C|GetMotionController _output_get) "None" "SnapToTarget" "SnapToTarget" "SnapToTarget" true)
  (Variables|Default|SetNotGrabbing true)
  (if (not true)
    (Components|Activation|SetActive (Variables|Components|GetMotionController_R) true false)))

(event EventTick
  (params (DeltaSeconds :type Float%20%28single-precision%29))
  (bind _endpoint (Variables|Default|GetEndPoint))
  (bind _returnvalue (Transformation|GetWorldLocation _endpoint))
  (CallFunction|Stretch)
  (bind (_hit _location _prim) (CallFunction|RaycasttoObject)) ; Raycast from Controller
  (CallFunction|TraceBeamMesh _hit _location _prim)
  (if (and (Variables|Default|GetTriggerPressed) (Variables|Default|GetHitOnce))
    (Physics|Components|PhysicsHandle|SetTargetLocation (Variables|Components|GetPhysicsHandle) (Transformation|GetWorldLocation (Variables|Default|GetEndPoint)))
    (Class|PrimitiveComponent|SetAngularDamping (Variables|Components|GetPhysics%20Object) 0.0)
    (if (Variables|Default|GetisExtending)
      (Physics|Components|PhysicsHandle|SetTargetLocation (Variables|Components|GetPhysicsHandle) (Math|Vector|Lerp(Vector) _returnvalue (+ _returnvalue (* (Math|Vector|Normalize (Math|Vector|GetForwardVector _endpoint)) (Variables|Default|GetRaycastLength))) (Variables|Default|GetArmLengthAlpha))))
    (Transformation|AddWorldOffset (Variables|Components|GetPhysics%20Object) (Variables|Default|GetLocation) false false)
    (Transformation|AddRelativeRotation (Variables|Components|GetPhysics%20Object) (Math|Rotator|MakeRotator 0.0 0.0 (Variables|Default|GetYaw)) false false)
    (Transformation|SetWorldScale3D (Variables|Components|GetPhysics%20Object) (Variables|Default|Getscale))))

(event Input|KeyboardEvents|MotionControllerRightTrigger
  (params (Key :type Key%20Structure :default "None"))
  (bind _hitonce (Variables|Default|GetHitOnce))
  (:Pressed
    (Variables|Default|SetTriggerPressed true)
    (if _hitonce
      (Physics|Components|PhysicsHandle|GrabComponentatLocationwithRotation (Variables|Components|GetPhysicsHandle) (Variables|Components|GetPhysics%20Object) "None" (Transformation|GetWorldLocation (Variables|Default|GetEndPoint)) (Math|Rotator|FindLookatRotation (Transformation|GetWorldLocation (Variables|Components|GetPhysics%20Object)) (Transformation|GetWorldLocation (Variables|/Game/Blueprint/control/MLTK/Common/BP_XRPawn.BP_XRPawn_C|GetMotionController (Variables|Default|GetXRPawn)))))))
  (:Released
    (Variables|Default|SetTriggerPressed false)
    (if _hitonce
      (Physics|Components|PhysicsHandle|ReleaseComponent (Variables|Components|GetPhysicsHandle))
      (CallFunction|DropObject (Variables|Components|GetPhysics%20Object)))))

(event Input|KeyboardEvents|MagicLeapRightHomeButton
  (params (Key :type Key%20Structure :default "None"))
  (:Pressed
    (bind _returnvalue (Game|GetCurrentLevelName true))
    (Game|OpenLevel(byName) (Utilities|String|StringToName _returnvalue))))

(fn ConstructionScript
  ;[1 1 1] Connect to veiw spline in viewport
)

(fn RaycasttoObject
  (bind _xrpawn (Variables|Default|GetXRPawn))
  (bind _motioncontroller (Variables|/Game/Blueprint/control/MLTK/Common/BP_XRPawn.BP_XRPawn_C|GetMotionController _xrpawn))
  (bind _returnvalue (Transformation|GetWorldLocation _motioncontroller))
  (if (Variables|Default|GetNotGrabbing)
    (bind (_outhit _returnvalue_2) (Collision|LineTraceByChannel _returnvalue (+ _returnvalue (* (Math|Vector|Normalize (Math|Vector|GetForwardVector _motioncontroller)) (Variables|Default|GetRaycastLength))) "TraceTypeQuery1" false (Variables|Default|GetActors%20to%20Ignore) "None"))
    (if _returnvalue_2
      (bind _output_get (Variables|Components|SetPhysics%20Object (.HitComponent (Collision|BreakHitResult _outhit))))
      (Rendering|Material|SetMaterial _output_get 0 "/Game/Blueprint/control/MLTK/ControllerPointer/Materials/M_TargetSelected.M_TargetSelected")
      (Variables|Default|SetHitOnce true)
      (bind _output_get_2 (Variables|Default|SetSelectedObject (.HitActor (Collision|BreakHitResult _outhit))))
      (if (Variables|Default|GetHitOnce)
        (Transformation|SetWorldLocation (Variables|Default|GetEndPoint) (Transformation|GetActorLocation _output_get_2) false false)
        (bind _output_get_3 (Variables|Default|SetIntScale (Transformation|GetWorldScale (Variables|Components|GetPhysics%20Object))))
        (Variables|Default|Setscale _output_get_3)
        (if (Variables|Default|GetTriggerPressed)
          (Variables|Default|SetNotGrabbing false)
          (else
            (Variables|Default|SetNotGrabbing true)))
        (return _returnvalue_2 (.Location (Collision|BreakHitResult _outhit)) (.HitComponent (Collision|BreakHitResult _outhit)) (.TraceEnd (Collision|BreakHitResult _outhit)))
        (else
          (Transformation|SetWorldLocation (Variables|Default|GetEndPoint) (.TraceEnd (Collision|BreakHitResult _outhit)) false false)))
      (elif (!= (Variables|Components|GetPhysics%20Object) 0)
        (Variables|Default|SetHitOnce false)
        (Rendering|Material|SetMaterial (Variables|Components|GetPhysics%20Object) 0 "/Game/Model/Level1/item/burger-box/source/box/material_0.material_0")
        (Variables|Components|SetPhysics%20Object 0)))))

(fn TraceBeamMesh
  (params (Hit :type Boolean) (Location :type Vector) (Prim :type Primitive%20Component%20Object%20Reference))
  (bind _spline1 (Variables|Components|GetSpline1))
  (bind _splinemesh (Variables|Components|GetSplineMesh))
  (bind _spline1_2 (Variables|Components|GetSpline1))
  (for _index (range 0 (- (Spline|GetNumberOfSplinePoints (Variables|Components|GetSpline1)) 2))
    (SplineMesh|SetForwardAxis _splinemesh "X" true)
    (if (Variables|Default|GetHitOnce)
      (Spline|SetLocationatSplinePoint _spline1 (+ _index 2) (Transformation|GetWorldLocation Prim) "World" true)
      (else
        (Spline|SetLocationatSplinePoint _spline1 (+ _index 2) (Math|Vector|MakeVector (Variables|Default|GetRaycastLength) 0.0 0.0) "Local" true)))
    (SplineMesh|SetStartandEnd _splinemesh (Spline|GetLocationatSplinePoint _spline1_2 _index "World") (Spline|GetTangentatSplinePoint _spline1_2 _index "World") (Spline|GetLocationatSplinePoint _spline1_2 (+ _index 2) "World") (Spline|GetTangentatSplinePoint _spline1_2 (+ _index 2) "World") true :!class /Script/Engine.SplineMeshComponent)
    (if (Variables|Default|GetHitOnce)
      _
      (else
        (Transformation|SetWorldLocation (Variables|Default|GetEndPoint) (Spline|GetLocationatSplinePoint _spline1_2 (+ _index 2) "World") false false)))
    (return Hit (Spline|GetLocationatSplinePoint _spline1_2 (+ _index 2) "World"))))

(fn Stretch
  (bind _xrpawn (Variables|Default|GetXRPawn))
  (bind _motioncontroller (Variables|/Game/Blueprint/control/MLTK/Common/BP_XRPawn.BP_XRPawn_C|GetMotionController _xrpawn))
  (bind _xr_camera (Variables|/Game/Blueprint/control/MLTK/Common/BP_XRPawn.BP_XRPawn_C|GetXR_Camera _xrpawn))
  (bind _returnvalue (Transformation|GetWorldLocation _motioncontroller))
  (bind _returnvalue_2 (Transformation|GetWorldLocation _xr_camera))
  (bind _returnvalue_3 (Math|Vector2D|MakeVector2D (.x _returnvalue) (.y _returnvalue)))
  (bind _returnvalue_4 (Math|Vector2D|MakeVector2D (.x _returnvalue_2) (.y _returnvalue_2)))
  (bind _returnvalue_5 (Math|Vector|Distance2D(Vector) _returnvalue_4 _returnvalue_3))
  (bind _returnvalue_6 (/ _returnvalue_5 1e+02))
  (bind _returnvalue_7 (Math|Float|Clamp(Float) _returnvalue_6 0.5 0.75))
  (if (>= _returnvalue_5 (Variables|Default|GetMaxArmLength))
    (Variables|Default|SetRaycastLength (Math|Float|Lerp 2.5e+02 5e+02 _returnvalue_7))
    (Variables|Default|SetisExtending true)
    (Variables|Default|SetArmLengthAlpha _returnvalue_7)
    (else
      (Variables|Default|SetRaycastLength 2.5e+02)
      (Variables|Default|SetisExtending false)
      (Variables|Default|SetArmLengthAlpha _returnvalue_7))))

(fn DropObject
  (params (Prim :type Primitive%20Component%20Object%20Reference))
  (Class|PrimitiveComponent|SetLinearDamping Prim 0.0)
  (Variables|Default|SetNotGrabbing true)
  (Variables|Default|SetHitOnce false)
  (Variables|Default|SetLocation "0, 0, 0")
  (Variables|Default|SetYaw 0.0)
  (Transformation|SetWorldScale3D (Variables|Components|GetPhysics%20Object) (Variables|Default|GetIntScale)))