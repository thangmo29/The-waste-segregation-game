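; BP_Spring is a draggable spring target that gives color and sound feedback to BP_ControlPointer interaction.
; Overlapping the pointer tints the Cube's dynamic material red and stores the controller; leaving restores white and clears it, each with a sound.
; Tick compares the Cube to its start location, using paired DoOnce gates to play one drag-begin sound on displacement and one drag-end sound once back with trigger released.
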(event OnComponentBeginOverlap(Cube)
  (params (OverlappedComponent :type Primitive%20Component%20Object%20Reference) (OtherActor :type Actor%20Object%20Reference) (OtherComp :type Primitive%20Component%20Object%20Reference) (OtherBodyIndex :type Integer) (bFromSweep :type Boolean) (SweepResult :type Hit%20Result%20Structure%20%28by%20ref%29))
  (bind _asbp_control_pointer (Utilities|Casting|CastToBP_ControlPointer OtherActor))
  (Variables|Default|SetBPController _asbp_control_pointer)
  (Rendering|Material|SetVectorParameterValue (Variables|Default|GetTarget%20Material) "Color" "(R=0.879623,G=0.020289,B=0.054480,A=1.000000)" :!class /Script/Engine.MaterialInstanceDynamic)
  (Audio|PlaySoundatLocation (Variables|Default|GetTarget%20Begin%20Sound) (Transformation|GetWorldLocation (Variables|Default|GetCube)) "0, 0, 0" 1.0 1.0 0.0 0 0 0))

(event OnComponentEndOverlap(Cube)
  (params (OverlappedComponent :type Primitive%20Component%20Object%20Reference) (OtherActor :type Actor%20Object%20Reference) (OtherComp :type Primitive%20Component%20Object%20Reference) (OtherBodyIndex :type Integer))
  (Variables|Default|SetBPController 0)
  (Rendering|Material|SetVectorParameterValue (Variables|Default|GetTarget%20Material) "Color" "(R=1.000000,G=1.000000,B=1.000000,A=1.000000)" :!class /Script/Engine.MaterialInstanceDynamic)
  (Audio|PlaySoundatLocation (Variables|Default|GetTarget%20End%20Sound) (Transformation|GetWorldLocation (Variables|Default|GetCube)) "0, 0, 0" 1.0 1.0 0.0 0 0 0))

(event EventBeginPlay
  (Variables|Default|SetInitialLocation (Transformation|GetWorldLocation (Variables|Default|GetCube)))
  (bind _outactors (Actor|GetAllActorsOfClass "/Game/MLTK/ControllerPointer/Blueprints/BP_ControlPointer.BP_ControlPointer_C"))
  (Variables|Default|SetBPController (Utilities|Array|Get(acopy) _outactors)))

(event EventTick
  (params (DeltaSeconds :type Float%20%28single-precision%29))
  (bind _bpcontroller (Variables|Default|GetBPController))
  (if (Math|Vector|Equal(Vector) (Variables|Default|GetInitialLocation) (Transformation|GetWorldLocation (Variables|Default|GetCube)) 1.0)
    (if (not (and (Variables|/Game/MLTK/ControllerPointer/Blueprints/BP_ControlPointer.BP_ControlPointer_C|GetTriggerPressed _bpcontroller) (!= _bpcontroller 0)))
      (Utilities|FlowControl|Sequence
        (:then_0
          (Utilities|FlowControl|DoOnce false :!label _label
            (:Completed
              (Audio|PlaySoundatLocation (Variables|Default|GetDrag%20End%20Sound) (Transformation|GetWorldLocation (Variables|Default|GetCube)) "0, 0, 0" 1.0 1.0 0.0 0 0 0))))
        (:then_1
          (goto _label_2 Reset))))
    (else
      (Variables|Default|SetDragging true)
      (Utilities|FlowControl|Sequence
        (:then_0
          (Utilities|FlowControl|DoOnce false :!label _label_2
            (:Completed
              (Audio|PlaySoundatLocation (Variables|Default|GetDrag%20Begin%20Sound) (Variables|Default|GetInitialLocation) "0, 0, 0" 1.0 1.0 0.0 0 0 0))))
        (:then_1
          (goto _label Reset))))))

(fn ConstructionScript
  (bind _returnvalue (Rendering|Material|CreateDynamicMaterialInstance (Variables|Default|GetCube) 0 "/Game/MLTK/ControllerPointer/Materials/M_Target.M_Target" "None" :!class /Script/Engine.PrimitiveComponent))
  (Variables|Default|SetTarget%20Material _returnvalue))