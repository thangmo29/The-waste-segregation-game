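; BP_Planes is a Magic Leap actor that visualizes detected real-world planes as static meshes.
; It requests planes asynchronously from its MagicLeapPlanes component every tick.
; Each successful result adds a static mesh component per plane, using its position and content orientation, with zero X thickness and Y/Z scaled from the plane's dimensions.
; The graph never removes or reuses earlier meshes, so components accumulate with every result.
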(event OnPlanesQueryResult(MagicLeapPlanes)
  (params (bSuccess :type Boolean) (Planes :type Array%20of%20Magic%20Leap%20Plane%20Result%20Structures) (Polygons :type Array%20of%20Magic%20Leap%20Plane%20Boundaries%20Structures))
  (bind (_x _y _z) (Math|Vector|BreakVector "100.000000,100.000000,100.000000"))
  (if bSuccess
    (for _array_element Planes
      (AddComponent|AddStaticMeshComponent false (Math|Transform|MakeTransform (.PlanePosition (Utilities|Struct|BreakMagicLeapPlaneResult _array_element)) (.ContentOrientation (Utilities|Struct|BreakMagicLeapPlaneResult _array_element)) (Math|Vector|MakeVector 0.0 (/ (.Y (Math|Vector2D|BreakVector2D (.PlaneDimensions (Utilities|Struct|BreakMagicLeapPlaneResult _array_element)))) _y) (/ (.X (Math|Vector2D|BreakVector2D (.PlaneDimensions (Utilities|Struct|BreakMagicLeapPlaneResult _array_element)))) _z)))))))

(event EventTick
  (params (DeltaSeconds :type Float%20%28single-precision%29))
  (Class|MagicLeapPlanesComponent|RequestPlanesAsync (Variables|Default|GetMagicLeapPlanes)))

(fn ConstructionScript)